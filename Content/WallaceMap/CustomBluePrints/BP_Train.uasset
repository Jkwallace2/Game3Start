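; Train hazard actor that travels back and forth along a spline, launching and killing characters it hits.
; A repeating 15-second loop, or debug key P, plays train audio, waits briefly at random, then flip-flops the Go timeline forward or backward.
; The timeline moves and rotates the Box along the spline, raised by its half-height.
; Box overlap launches characters along the impact normal with massive environmental damage, playing a 2D horn for the player.
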(event OnComponentBeginOverlap(Box)
  (params (OverlappedComponent :type Primitive%20Component%20Object%20Reference) (OtherActor :type Actor%20Object%20Reference) (OtherComp :type Primitive%20Component%20Object%20Reference) (OtherBodyIndex :type Integer) (bFromSweep :type Boolean) (SweepResult :type Hit%20Result%20Structure%20%28by%20ref%29))
  (if (== OtherActor (Game|Player|GetPlayerPawn 0))
    (Audio|PlaySound2D "/Game/WallaceMap/CustomBluePrints/train-horn-meme_v6N3591.train-horn-meme_v6N3591" 0.5 1.0 0.0 0 0))
  (bind _ascharacter (Utilities|Casting|CastToCharacter OtherActor))
  (Character|LaunchCharacter _ascharacter (* (.ImpactNormal (Collision|BreakHitResult SweepResult)) 2e+03) true true)
  (Game|Damage|ApplyDamage OtherActor 1e+04 0 0 "/Engine/EngineDamageTypes/DmgTypeBP_Environmental.DmgTypeBP_Environmental_C"))

(event Custom|Traindo
  (bind _spline (Variables|Default|GetSpline))
  (bind _box (Variables|Default|GetBox))
  ;[0.15 0.15 0.15 0.5] why no you stupid b******ard, Attenuation refuses to work
  (Audio|Components|Audio|Play (Variables|Default|GetSC_Train) 0.0)
  (Utilities|FlowControl|Delay (Math|Random|RandomFloatinRange 0.5 2.0))
  (Utilities|FlowControl|FlipFlop
    (:A
      (bind _newtrack_0 (Timeline|Go PlayFromStart)
        (:Update
          (Transformation|SetWorldLocationAndRotation _box (+ (.Location (Math|Transform|BreakTransform (Spline|GetTransformatDistanceAlongSpline _spline (* _newtrack_0 (Spline|GetSplineLength _spline)) "World" false))) (* (Components|Box|GetScaledBoxExtent _box) "0.000000,0.000000,1.000000")) (.Rotation (Math|Transform|BreakTransform (Spline|GetTransformatDistanceAlongSpline _spline (* _newtrack_0 (Spline|GetSplineLength _spline)) "World" false))) false false))))
    (:B
      (Timeline|Go ReverseFromEnd))))

(event EventBeginPlay
  (CallFunction|Traindo :!label _label)
  (Utilities|FlowControl|Delay 15.0)
  (goto _label))

(event Collision|EventActorBeginOverlap
  (params (OtherActor :type Actor%20Object%20Reference)))

(event EventTick
  (params (DeltaSeconds :type Float%20%28single-precision%29)))

(event Input|KeyboardEvents|DebugKeyP
  (params (Key :type Key%20Structure) (ActionValue :type Input%20Action%20Value%20Structure))
  (:Pressed
    (CallFunction|Traindo)))

(fn ConstructionScript)