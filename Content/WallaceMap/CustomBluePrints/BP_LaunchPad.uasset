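; Launch pad that throws any overlapping Character toward a target Scene component, with a rocket launcher sound.
; On BeginPlay it raises LaunchSpeed until a projectile arc to the target is found, then aims the Arrow along it.
; It then spawns a NavLinkProxy from the pad-target midpoint, leaving its links unconfigured.
; Sphere overlap re-solves the toss from a lowered start, falling back to the Arrow's direction at LaunchSpeed.
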(event `set nav link`
  (`|SpawnActorFromClass` "/Script/AIModule.NavLinkProxy" (`KismetMathLibrary.MakeTransform` (+ (/ (- (`SceneComponent.RelativeLocation` (`self.Scene`)) (`SceneComponent.RelativeLocation` (`self.Sphere`))) 2.0) (`SceneComponent.RelativeLocation` (`self.Sphere`)))) "Undefined" "MultiplyWithRoot" null null))

(event `self.ReceiveBeginPlay`
  (bind (_tossvelocity _returnvalue) (`GameplayStatics.BlueprintSuggestProjectileVelocity` (`SceneComponent.K2_GetComponentLocation` (`self.Sphere`)) (`SceneComponent.K2_GetComponentLocation` (`self.Scene`)) (`self.Launch Speed`) 0.0 "DoNotTrace" 50.0 (`self.Favor High Arc`) :!label _label))
  (if _returnvalue
    (`SceneComponent.K2_SetWorldRotation` (`self.Arrow`) (`KismetMathLibrary.Conv_VectorToRotator` _tossvelocity) false false)
    (`SceneComponent.K2_SetWorldRotation` (`self.Arrow`) (`KismetMathLibrary.Conv_VectorToRotator` _tossvelocity) false false)
    (`self.set nav link`)
    (else
      (set `self.Launch Speed` (+ (`self.Launch Speed`) 1000.0))
      (goto _label))))

(event `self.Sphere.OnComponentBeginOverlap`
  (params (OverlappedComponent :type "PrimitiveComponent Object Reference") (OtherActor :type "Actor Object Reference") (OtherComp :type "PrimitiveComponent Object Reference") (OtherBodyIndex :type Integer) (bFromSweep :type Boolean) (SweepResult :type "HitResult Structure (by ref)"))
  (bind _ascharacter (cast `Character` OtherActor))
  (`GameplayStatics.PlaySoundAtLocation` "/Game/WallaceMap/CustomBluePrints/Audio/00_Toys/Toy_RocketLauncher.Toy_RocketLauncher" (`SceneComponent.K2_GetComponentLocation` (`self.Sphere`)) (struct) 1.0 1.0 0.0 "/Game/FPS/Sound/AttenuationPresets/ATT_Default.ATT_Default" null null null)
  (bind (_tossvelocity _returnvalue) (`GameplayStatics.BlueprintSuggestProjectileVelocity` (- (`SceneComponent.K2_GetComponentLocation` (`self.Sphere`)) (0.0 0.0 200.0)) (`SceneComponent.K2_GetComponentLocation` (`self.Scene`)) (`self.Launch Speed`) 0.0 "DoNotTrace" 0.0 (`self.Favor High Arc`)))
  ; wtf?
  (if _returnvalue
    (`Character.LaunchCharacter` _ascharacter _tossvelocity true true)
    (else
      (`Character.LaunchCharacter` _ascharacter (* (`SceneComponent.GetForwardVector` (`self.Arrow`)) (`self.Launch Speed`)) true true))))

(fn `UserConstructionScript`)