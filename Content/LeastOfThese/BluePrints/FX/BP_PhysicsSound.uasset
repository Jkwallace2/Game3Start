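; Short-lived actor that plays a material-specific sound at a physics impact, then destroys itself.
; On BeginPlay it discards impacts below MinForce, scales volume by strength, then runs GetInfo and Execute.
; GetInfo, overridable by children, reads the hit and maps its physical material's array index to a sound enum.
; Execute plays the attenuated sound and optionally spawns debug Niagara FX, a decal and controller rumble.
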(event `self.ReceiveBeginPlay`
  (bind _impactstrength (`self.ImpactStrength`))
  (if (>= _impactstrength (`self.MinForce`))
    (set `self.LocalVolume` (`KismetMathLibrary.MapRangeClamped` _impactstrength 500.0 4000.0 0.01 2.0))
    ; Maybe i want to change how we get sound info, Children can override but execute is the same
    (`self.GetInfo`)
    (`self.Execute`)
    (else
      (`self.K2_DestroyActor`))))

(event `Execute`
  (`|ExecutionSequence`
    (:`then_0`
      (switch `/Game/LeastOfThese/BluePrints/FX/PhysMats/Enum_PhysSounds` (`self.Material`)
        (:`NewEnumerator0`
          (set `self.Sound` "/Game/DoubleAction/FirstPerson/Audio/FootStep.FootStep"))
        (:`NewEnumerator1`
          (set `self.Sound` "/Game/Audio/GrassSteps/grassStep_Cue.grassStep_Cue"))
        (:`NewEnumerator2`
          (set `self.Sound` "/Game/Audio/SFX/WallaceToySFX/01_Crystal/Crystal_ImpactClosed.Crystal_ImpactClosed"))
        (:`NewEnumerator3`
          (set `self.Sound` "/Game/Audio/SFX/Phisics/Metal/SawImpactD.SawImpactD"))
        (:`NewEnumerator4`
          (set `self.Sound` "/Game/Audio/SFX/Phisics/Flesh/Cantaloupe_Gore2.Cantaloupe_Gore2"))
        (:`NewEnumerator5`
          (set `self.Sound` "/Game/Audio/SFX/WallaceToySFX/00_Toys/Toy_BoltSlide.Toy_BoltSlide"))
        (:`NewEnumerator6`
          (set `self.Sound` "/Game/Audio/SFX/WallaceToySFX/05_GameSounds/Game_Pickup.Game_Pickup"))
        (:`NewEnumerator7`
          (set `self.Sound` "/Game/DoubleAction/FirstPerson/Audio/FootStep.FootStep"))))
    (:`then_1`
      (`GameplayStatics.PlaySoundAtLocation` (`self.Sound`) (`self.SoundLocation`) (struct) (`self.LocalVolume`) 1.0 0.0 "/Game/Audio/Attenuation/SA_PhysicsImpact.SA_PhysicsImpact" null null null)
      (if (`self.AlsoDoFX`)
        (`NiagaraFunctionLibrary.SpawnSystemAtLocation` "/Game/LeastOfThese/FX/NS_DebugNormal.NS_DebugNormal" (`self.SoundLocation`) (`self.SoundRotation`)))
      (if (`self.AlsoDoDecal`)
        (`|SpawnActorFromClass` "/Game/LeastOfThese/BluePrints/FX/BP_PhysicsDecal.BP_PhysicsDecal_C" (`KismetMathLibrary.MakeTransform` (`self.SoundLocation`) (`self.SoundRotation`) (`KismetMathLibrary.Conv_DoubleToVector` (`self.BaseFxSize`))) "Undefined" "MultiplyWithRoot" null 3.0 1.0 (`self.UseXVectorForDecal`) null))
      (if (`self.AlsoDoRumble`)
        ; TEST THIS
        (`GameplayStatics.SpawnForceFeedbackAtLocation` "/Game/LeastOfThese/BluePrints/FX/Rumble/FFE_Crystal.FFE_Crystal" (`self.SoundLocation`) (struct) false 1.0 0.0 "/Game/LeastOfThese/BluePrints/FX/Rumble/FFA_SmallPhys.FFA_SmallPhys"))
      (`self.K2_DestroyActor`))))

(event `GetInfo`
  (bind (_inhit_bblockinghit _inhit_binitialoverlap _inhit_time _inhit_distance _inhit_location _inhit_impactpoint _inhit_normal _inhit_impactnormal _inhit_physmat) (`GameplayStatics.BreakHitResult` (`self.InHit`)))
  ; If we do not want to use tthe infro from a ray cast override this in children
  (set `self.SoundLocation` _inhit_impactpoint)
  (set `self.SoundRotation` (`KismetMathLibrary.Conv_VectorToRotator` _inhit_normal))
  (`self.BreakKnownPhysMats` _inhit_physmat))

(fn `BreakKnownPhysMats`
  (params (PhysMat :type "Object Object Reference"))
  (returns (PhysicalMaterial :type "/Game/LeastOfThese/BluePrints/FX/PhysMats/Enum_PhysSounds Enum"))
  (locals (PhysSounds :type "/Game/LeastOfThese/BluePrints/FX/PhysMats/Enum_PhysSounds Enum") (PhysMats :type "Array of Object Object Reference"))
  (bind _physmats (`local.PhysMats`))
  (for (_array_element _array_index) _physmats
    (if (== PhysMat _array_element)
      (bind _output_get (set `local.PhysSounds` (cast `/Game/LeastOfThese/BluePrints/FX/PhysMats/Enum_PhysSounds` (`KismetMathLibrary.Conv_IntToByte` _array_index))))
      (break)))
  (if (== _array_index (`KismetArrayLibrary.Array_Length` _physmats))
    (`KismetSystemLibrary.PrintString` "castFailed"))
  (`KismetSystemLibrary.PrintString` (`KismetSystemLibrary.GetDisplayName` PhysMat))
  (bind _output_get_2 (set `self.Material` _output_get))
  (return _output_get_2))

(fn `UserConstructionScript`)