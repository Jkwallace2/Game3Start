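; Base enemy character that can pick up, carry and throw grenades, with a suicide variant that explodes when damaged.
; A carried bomb's fuse counts down on Tick with material, sound and sweat cues, triggering a panic throw or explosion.
; Throws spawn homing grenades, normally after a sphere trace confirms the player.
; Damage notifies the AI controller or ragdolls the enemy; patrol spline helpers and empty override events round it out.
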(event `self.ReceiveBeginPlay`
  (if (not (`self.Suislide?`))
    (`ActorComponent.K2_DestroyComponent` (`self.Audio`)))
  (set `self.OgMaterial` (`PrimitiveComponent.GetMaterial` (`self.Mesh`) 0)))

(event `Attack`)

(event `Ranged attack`
  (params (Target :type "Vector Structure") (Actor :type "Actor Object Reference"))
  (`KismetSystemLibrary.PrintString` "Tossing Bomb" true true (struct :`R` 1.0 :`G` 0.97268 :`B` 0.721657 :`A` 1.0))
  (`self.ThowNewBomb` Target Actor)
  (`KismetSystemLibrary.Delay` 0.01)
  (`self.RangeAttackFInished`))

(event `GetAggro`
  (set `self.Aggroed` true)
  (`self.CustomWhenAgroed`))

(event `CustomWhenAgroed`)

(event `loseAggro`)

(event `InstaSplode`
  (bind _returnvalue (`SceneComponent.K2_GetComponentLocation` (`self.Sphere`)))
  ; Suicide death
  (`/Engine/EditorBlueprintResources/StandardMacros.DoOnce` false
    (:`Completed`
      (`self.Lose Bomb`)
      (set `self.Fuse` 0)
      (set `self.Health` 0.0)
      (`KismetSystemLibrary.DelayUntilNextTick`)
      (`self.Ragdoll` _returnvalue (0.0 0.0 -1.0))
      (`|SpawnActorFromClass` "/Game/Blueprints/BP_Explosion.BP_Explosion_C" (`KismetMathLibrary.MakeTransform` _returnvalue) "Undefined" "MultiplyWithRoot" null self (`self.GetInstigator`)))))

(event `Set Speed`
  (params (NewSpeed :type "Float (double-precision)"))
  (set `CharacterMovementComponent.MaxWalkSpeed` NewSpeed (`self.CharacterMovement`)))

(event `self.ReceiveAnyDamage`
  (params (Damage :type "Float (single-precision)") (DamageType :type "DamageType Object Reference") (InstigatedBy :type "Controller Object Reference") (DamageCauser :type "Actor Object Reference"))
  (if (`self.Suislide?`)
    (`self.InstaSplode`)
    (elif (`self.IsHoldingBomb`)
      (`self.InstaSplode`)
      (else
        (`KismetSystemLibrary.DelayUntilNextTick`)
        (message `/Game/AI_Blueprints/BPI_BetterAiCommunication.BPIDamage` (`self.AIC`) Damage (`self.Health`))))))

(event `self.ReceivePointDamage`
  (params (Damage :type "Float (single-precision)") (DamageType :type "DamageType Object Reference") (HitLocation :type "Vector Structure") (HitNormal :type "Vector Structure") (HitComponent :type "PrimitiveComponent Object Reference") (BoneName :type Name) (ShotFromDirection :type "Vector Structure") (InstigatedBy :type "Controller Object Reference") (DamageCauser :type "Actor Object Reference") (HitInfo :type "HitResult Structure (by ref)"))
  (bind _audio (`self.Audio`))
  (if (`self.Suislide?`)
    (`self.InstaSplode`)
    (else
      (`KismetSystemLibrary.PrintText` (`|FormatText` "{inst} Damaged us for {dmg}" InstigatedBy Damage) true true (struct :`R` 1.0 :`G` 0.126631 :`A` 1.0))
      (bind _output_get (set `self.Health` (- (`self.Health`) Damage)))
      (if (<= _output_get 0.0)
        (`/Engine/EditorBlueprintResources/StandardMacros.IsValid` _audio
          (:`Is Valid`
            (`AudioComponent.Stop` _audio))
          (:`Is Not Valid`
            _))
        (`KismetSystemLibrary.DelayUntilNextTick`)
        (if (`self.IsHoldingBomb`)
          (`self.PanicTrouw`))
        (`self.Ragdoll` HitLocation (* ShotFromDirection (* (`KismetMathLibrary.MapRangeClamped` Damage 0.0 200.0 0.0 1000.0) 1.0)))
        (elif (<= (`self.Health`) 30.0)
          (`self.Low Health`))))))

(event `Low Health`
  (`SceneComponent.SetVisibility` (`self.Billboard`) true true)
  (message `/Game/AI_Blueprints/BPI_BetterAiCommunication.IAmLowHealth` (`self.AIC`)))

(event `/Game/AI_Blueprints/BPI_BetterAiCommunication.IAmLowHealth`
  (`SceneComponent.SetVisibility` (`self.Billboard`) false true :!label _label))

(event `self.ReceiveRadialDamage`
  (params (DamageReceived :type "Float (single-precision)") (DamageType :type "DamageType Object Reference") (Origin :type "Vector Structure") (HitInfo :type "HitResult Structure (by ref)") (InstigatedBy :type "Controller Object Reference") (DamageCauser :type "Actor Object Reference"))
  (if (`self.Suislide?`)
    (`self.InstaSplode`)
    (else
      (bind _output_get (set `self.Health` (- (`self.Health`) DamageReceived)))
      (if (<= _output_get 0.0)
        (`self.Ragdoll` Origin (0.0 0.0 2000.0))
        (elif (<= (`self.Health`) 30.0)
          (`self.Low Health`))))))

(event `IAmBrave`
  (if (not (`self.Suislide?`))
    (goto _label)))

(event `Ragdoll`
  (params (Origin :type "Vector Structure") (Impulse :type "Vector Structure"))
  (bind _returnvalue (`GameplayStatics.GetPlayerPawn` 0))
  (bind _mesh (`self.Mesh`))
  (bind _audio (`self.Audio`))
  ; Death
  (`/Engine/EditorBlueprintResources/StandardMacros.IsValid` _audio
    (:`Is Valid`
      (`AudioComponent.Stop` _audio))
    (:`Is Not Valid`
      _))
  (`SceneComponent.SetVisibility` (`self.Billboard`) false false)
  (`/Engine/EditorBlueprintResources/StandardMacros.DoOnce` false
    (:`Completed`
      (`self.Special Death`)
      (if (`self.IsHoldingBomb`)
        (`self.Ranged attack` (`self.K2_GetActorLocation` _returnvalue) _returnvalue))
      (`PrimitiveComponent.SetSimulatePhysics` _mesh true)
      (`self.Lose Bomb`)
      (`PrimitiveComponent.AddImpulseAtLocation` _mesh Impulse Origin "head")
      (`CharacterMovementComponent.DisableMovement` (`self.CharacterMovement`))
      (`PrimitiveComponent.SetCollisionEnabled` (`self.CapsuleComponent`) "NoCollision")
      (`KismetSystemLibrary.Delay` 8.0)
      (`PrimitiveComponent.SetCollisionResponseToChannel` (`self.Mesh`) "ECC_Destructible" "ECR_Ignore")
      (`KismetSystemLibrary.Delay` 1.0)
      (`self.K2_DestroyActor`))))

(event `Special Death`)

(event `GetBomb`
  (`self.IAmBrave`)
  (set `self.IsHoldingBomb` true)
  (if (<= (`self.Health`) 30.0)
    (set `self.Health` 40.0))
  (`SceneComponent.SetVisibility` (`self.Sphere`) true false))

(event `/Game/AI_Blueprints/BPI_BetterAiCommunication.GetAIC`
  (params (AIC :type "AIController Object Reference"))
  (set `self.AIC` AIC))

(event `Lose Bomb`
  (set `self.IsHoldingBomb` false)
  (`SceneComponent.SetVisibility` (`self.Sphere`) false false))

(event `self.ReceiveTick`
  (params (DeltaSeconds :type "Float (single-precision)"))
  (`self.BombTick`))

(event `ReportFuse`
  (params (Fuse :type Integer))
  (bind _sphere (`self.Sphere`))
  ; Explode if overcooked
  (if (<= Fuse 0)
    ;; only explode if i am still holding bomb
    (if (`self.IsHoldingBomb`)
      (`self.Lose Bomb`)
      (if (`self.Suislide?`)
        (`self.Ragdoll` (0.0 0.0 0.0)))
      (`|SpawnActorFromClass` "/Game/Blueprints/BP_Explosion.BP_Explosion_C" (`KismetMathLibrary.MakeTransform` (+ (`SceneComponent.K2_GetComponentLocation` _sphere) (`SceneComponent.GetForwardVector` _sphere)) (`SceneComponent.K2_GetComponentRotation` _sphere)) "Undefined" "MultiplyWithRoot" null self (`self.GetInstigator`))
      (else
        (`self.Lose Bomb`)))
    (else
      (`|ExecutionSequence`
        (:`then_0`
          (if (<= Fuse 20)
            (`NiagaraFunctionLibrary.SpawnSystemAtLocation` "/Game/VFX/NS_Sweat.NS_Sweat" (`SceneComponent.GetSocketLocation` (`self.Mesh`) "Head"))))
        (:`then_1`
          (if (and (<= Fuse 15) (!= (`self.Suislide?`) true))
            (`self.PanicTrouw`)))))))

(event `BombTick`
  ; Explode if overcooked
  (if (`self.IsHoldingBomb`)
    (`KismetSystemLibrary.Delay` 0.1)
    (bind _result (`/Engine/EditorBlueprintResources/StandardMacros.DecrementInt` (`self.Fuse`))
      (:`  `
        (`self.FuseFX` _result)
        (`self.ReportFuse` _result)))))

(event `PanicTrouw`
  (bind _returnvalue (`GameplayStatics.GetPlayerPawn` 0))
  ; Explode if overcooked
  (`KismetSystemLibrary.PrintString` "PanicThrow" true true (struct :`R` 1.0 :`G` 0.100343 :`A` 1.0))
  (`self.ThowNewBomb` (`self.K2_GetActorLocation` _returnvalue) _returnvalue true))

(event `FuseFX`
  (params (Fuse :type Integer))
  (bind _returnvalue (`KismetMathLibrary.MapRangeClamped` (`KismetMathLibrary.Conv_IntToDouble` Fuse) 0.0 29.0 1.0))
  ; Explode if overcooked
  (`MeshComponent.SetScalarParameterValueOnMaterials` (`self.Sphere`) "Fuse" _returnvalue)
  (if (== (mod Fuse 2) 0)
    (bind _returnvalue_2 (`GameplayStatics.SpawnSoundAttached` "/Game/Audio/SC_TickingBomb.SC_TickingBomb" (`self.Sphere`) "None" (0.0 0.0 0.0) (struct) "KeepRelativeOffset" false 1.0 1.0 0.0 null null))
    (`/Engine/EditorBlueprintResources/StandardMacros.IsValid` _returnvalue_2
      (:`Is Valid`
        (`AudioParameterControllerInterface.SetFloatParameter` _returnvalue_2 "Blend" _returnvalue)))))

(event `Prime`)

(fn `GetIdealRange`
  (returns (AttackRadius :type "Float (double-precision)") (StrafeRadius :type "Float (double-precision)"))
  (return (`self.Attack Radius`) (`self.Strafe Radius`)))

(fn `GetNextPatrolPointLocation`
  (returns (Location :type "Vector Structure"))
  (`/Engine/EditorBlueprintResources/StandardMacros.IsValid` (`self.PatrolRoute`)
    (:`Is Valid`
      ; update next point
      (bind _output_get (set `self.PatrolPointIndex` (+ (`self.PatrolPointIndex`) (`self.PatrolRouteDIrection`))))
      (if (or (>= (`self.PatrolPointIndex`) (- (`SplineComponent.GetNumberOfSplinePoints` (`/Game/AI_Blueprints/BP_PatrolRoute.Spline` (`self.PatrolRoute`))) 1)) (<= (`self.PatrolPointIndex`) 0))
        (set `self.PatrolRouteDIrection` (* (`self.PatrolRouteDIrection`) -1)))
      (return (`SplineComponent.GetLocationAtSplinePoint` (`/Game/AI_Blueprints/BP_PatrolRoute.Spline` (`self.PatrolRoute`)) _output_get "World")))
    (:`Is Not Valid`
      (`KismetSystemLibrary.PrintString` "No Route assigned"))))

(fn `PickupBomb`
  (returns (GotBomb :type Boolean))
  (locals (NewLocalVar :type "Array of EObjectTypeQuery Enum"))
  (bind _returnvalue (`SceneComponent.K2_GetComponentLocation` (`self.CapsuleComponent`)))
  (if (not (`self.IsHoldingBomb`))
    (bind _outhits (`KismetSystemLibrary.SphereTraceMultiForObjects` _returnvalue _returnvalue 300.0 (`local.NewLocalVar`)))
    (for _array_element _outhits
      (bind (_bblockinghit _binitialoverlap _time _distance _location _impactpoint _normal _impactnormal _physmat _hitactor) (`GameplayStatics.BreakHitResult` _array_element))
      (bind _asbp_grenade_safe (cast `/Game/Blueprints/levelStuff/BP_GrenadeSafe` _hitactor)
        (:`then`
          (bind _litfuse (`/Game/Blueprints/levelStuff/BP_Grenade.LitFuse` _asbp_grenade_safe))
          (set `self.Fuse` _litfuse)
          (`KismetSystemLibrary.PrintString` (`KismetStringLibrary.Conv_IntToString` _litfuse) true true (struct :`R` 1.0 :`G` 0.791726 :`A` 1.0) 60.0)
          (`self.K2_DestroyActor` _asbp_grenade_safe))
        (:`CastFailed`
          (bind _asbp_grenade (cast `/Game/Blueprints/levelStuff/BP_Grenade` _hitactor))
          (bind _litfuse_2 (`/Game/Blueprints/levelStuff/BP_Grenade.LitFuse` _asbp_grenade))
          (set `self.Fuse` _litfuse_2)
          (`KismetSystemLibrary.PrintString` (`KismetStringLibrary.Conv_IntToString` _litfuse_2) true true (struct :`R` 1.0 :`G` 0.791726 :`A` 1.0) 60.0)
          (`self.K2_DestroyActor` _asbp_grenade)))
      (`self.GetBomb`)
      (return true)))
  (return false))

(fn `ProfileBombs`
  (`KismetSystemLibrary.PrintString` "Testing Bombs in radius"))

(fn `ThowNewBomb`
  (params (Aim :type "Vector Structure") (TargetActor :type "Actor Object Reference") (IgnoreAllThrow :type Boolean))
  (bind _returnvalue_location (`KismetMathLibrary.BreakTransform` (`self.GetTransform`)))
  (bind _returnvalue (`SceneComponent.K2_GetComponentLocation` (`self.CapsuleComponent`)))
  (bind _returnvalue_2 (* (`KismetMathLibrary.GetForwardVector` (`KismetMathLibrary.FindLookAtRotation` _returnvalue (+ Aim (`KismetMathLibrary.MakeVector` 0.0 0.0 (`KismetMathLibrary.MapRangeUnclamped` (`KismetMathLibrary.Vector_Distance` _returnvalue Aim) 0.0 800.0 50.0 100.0))))) 1.0))
  (if IgnoreAllThrow
    (`|SpawnActorFromClass` "/Game/Blueprints/levelStuff/BP_Grenade.BP_Grenade_C" (`KismetMathLibrary.MakeTransform` (+ _returnvalue_location (* _returnvalue_2 40.0)) (`KismetMathLibrary.Conv_VectorToRotator` _returnvalue_2)) "Undefined" "MultiplyWithRoot" null (* (`KismetMathLibrary.Conv_IntToDouble` (`self.Fuse`)) 0.1) 3000.0 false TargetActor (`self.BombToThrow`) self null :!label _label)
    (`self.Lose Bomb`)
    (else
      ; Dont hit buddies
      (bind _outhit (`KismetSystemLibrary.SphereTraceSingleByProfile` (`SceneComponent.GetSocketLocation` (`self.Mesh`) "Head") Aim 60.0 "BlockAll"))
      (if (== (`.HitActor` (`GameplayStatics.BreakHitResult` _outhit)) (`GameplayStatics.GetPlayerPawn` 0))
        (`KismetSystemLibrary.PrintString` "EMEMY TROWING BALL" true true (struct :`R` 1.0 :`B` 0.093081 :`A` 1.0))
        (goto _label)))))

(fn `UserConstructionScript`
  (`SceneComponent.SetVisibility` (`self.Sphere`) false false))