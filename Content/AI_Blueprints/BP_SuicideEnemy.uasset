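; Suicide bomber enemy, a child Blueprint that primes a bomb and chases the player with it.
; Its construction script overrides fuse, health, attack and strafe radii and a Suislide flag before running the parent's.
; Prime fires once, setting IsHoldingBomb and playing audio if the enemy is alive.
; Tick runs BombTick and, while the bomb is held, reissues AI MoveTo toward the player pawn every frame.
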(event `self.ReceiveBeginPlay`
  (`SceneComponent.SetVisibility` (`self.Sphere`) true false)
  (`parent.ReceiveBeginPlay`))

(event `self.ReceiveTick`
  (params (DeltaSeconds :type "Float (single-precision)"))
  (bind _returnvalue (`GameplayStatics.GetPlayerPawn` 0))
  (bind _returnvalue_location (`KismetMathLibrary.BreakTransform` (`self.GetTransform` _returnvalue)))
  (`self.BombTick`)
  (if (`self.IsHoldingBomb`)
    (`|AIMoveTo` (`self.CharacterMovement`) null _returnvalue_location _returnvalue)))

(event `self.Prime`
  (`/Engine/EditorBlueprintResources/StandardMacros.DoOnce` false
    (:`Completed`
      (if (> (`self.Health`) 0.0)
        (set `self.IsHoldingBomb` true)
        (`AudioComponent.Play` (`self.Audio`) 0.0)))))

(fn `UserConstructionScript`
  (set `self.Fuse` 70)
  (set `self.Health` 40.0)
  (set `self.Suislide?` true)
  (set `self.Attack Radius` 100.0)
  (set `self.Strafe Radius` 800.0)
  (`parent.UserConstructionScript`))