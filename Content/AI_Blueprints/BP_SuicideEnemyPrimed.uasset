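; BP_SuicideEnemyPrimed is a suicide enemy variant that begins play already holding a bomb.
; On BeginPlay it runs the parent logic, then overrides the fuse value, shows the Sphere component and sets the bomb-holding flag.
; Overlap and construction pass straight to the parent, and Tick is disabled, so any further behavior is inherited.
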(event `self.ReceiveBeginPlay`
  (`parent.ReceiveBeginPlay`)
  (set `self.Fuse` 50)
  (`SceneComponent.SetVisibility` (`self.Sphere`) true false)
  (set `self.IsHoldingBomb` true))

(event `self.ReceiveActorBeginOverlap`
  (params (OtherActor :type "Actor Object Reference"))
  (`parent.ReceiveActorBeginOverlap` OtherActor))

(fn `UserConstructionScript`
  (`parent.UserConstructionScript`))