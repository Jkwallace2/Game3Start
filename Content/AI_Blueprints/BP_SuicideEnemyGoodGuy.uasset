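; BP_SuicideEnemyGoodGuy is a bomb-carrying suicide AI that hunts other enemies and blows itself up on reaching them.
; On BeginPlay it plays audio, sets its fuse, shows a sphere, flags the bomb as held and picks the nearest other BP_EnemyBase actor.
; Tick drives AIMoveTo toward that target, calling InstaSplode on arrival, and searches again whenever the target is invalid.
; The parent's Tick call is disabled.
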(event `self.ReceiveActorBeginOverlap`
  (params (OtherActor :type "Actor Object Reference"))
  (`parent.ReceiveActorBeginOverlap` OtherActor))

(event `self.ReceiveBeginPlay`
  (`parent.ReceiveBeginPlay`)
  (`AudioComponent.Play` (`self.Audio`) 0.0)
  (`self.FindTarget`)
  (set `self.Fuse` 30)
  (`SceneComponent.SetVisibility` (`self.Sphere`) true false)
  (set `self.IsHoldingBomb` true))

(event `FindTarget`
  (bind _outactors (`GameplayStatics.GetAllActorsOfClass` "/Game/AI_Blueprints/BP_EnemyBase.BP_EnemyBase_C"))
  (`KismetArrayLibrary.Array_RemoveItem` _outactors self)
  (set `self.Target` (`.ReturnValue` (`GameplayStatics.FindNearestActor` (`SceneComponent.K2_GetComponentLocation` (`self.CapsuleComponent`)) _outactors))))

(event `self.ReceiveTick`
  (params (DeltaSeconds :type "Float (single-precision)"))
  (`/Engine/EditorBlueprintResources/StandardMacros.IsValid` (`self.Target`)
    (:`Is Valid`
      (`|AIMoveTo` self (0.0 0.0 0.0) (`self.Target`) 50.0
        (:`OnSuccess`
          (`self.InstaSplode`))))
    (:`Is Not Valid`
      (`self.FindTarget`))))

(fn `UserConstructionScript`
  (`parent.UserConstructionScript`))