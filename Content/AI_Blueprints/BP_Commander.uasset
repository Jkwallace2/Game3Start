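; BP_Commander is a ranged, super-aggressive enemy AI variant with self-preservation, built on a parent class that it configures through its construction script.
; The construction script sets its name, health, attack and strafe radii, and thrown bomb type, then runs the parent's setup.
; Becoming aggroed reveals a cube component.
; Its special death runs a delayed, counted loop that plays a bubble sound and launches fused grenades from the capsule in random directions.
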(event `self.Special Death`
  (bind _returnvalue (`SceneComponent.K2_GetComponentLocation` (`self.CapsuleComponent`)))
  (`KismetSystemLibrary.Delay` 0.1)
  (while (> (`self.i`) 0)
    (`/Engine/EditorBlueprintResources/StandardMacros.DecrementInt` (`self.i`)
      (:`  `
        (`GameplayStatics.PlaySoundAtLocation` "/Game/Audio/bubble2.bubble2" _returnvalue (struct) 2.0 1.0 0.0 null null null null)
        (`|SpawnActorFromClass` "/Game/Blueprints/levelStuff/BP_Grenade.BP_Grenade_C" (`KismetMathLibrary.MakeTransform` _returnvalue (`KismetMathLibrary.RandomRotator` false)) "Undefined" "MultiplyWithRoot" null 2.0 1000.0 false null "NewEnumerator3" null null)
        (`KismetSystemLibrary.Delay` 0.21)))))

(event `self.CustomWhenAgroed`
  (`SceneComponent.SetVisibility` (`self.Cube`) true false))

(fn `UserConstructionScript`
  (set `self.BombToThrow` "NewEnumerator3")
  (set `self.Attack Radius` 800.0)
  (set `self.Strafe Radius` 1500.0)
  (set `self.AmIRangedEnemy` true)
  (set `self.SuperAgressive` true)
  (set `self.SelfPreservation` true)
  (set `self.Health` 80.0)
  (set `self.FirstName` "John")
  (set `self.LastName` "KYS")
  (`parent.UserConstructionScript`))