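; AI pawn Blueprint that displays its name by joining first and last name into a text element.
; The text is set on BeginPlay and refreshed through the UpdateName event.
; An unconnected AI Move To loop, which would retarget player controller 0 one second after each success or failure, never runs.
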(event `self.ReceiveBeginPlay`
  (`TextRenderComponent.K2_SetText` (`self.AI FirstName`) (`KismetTextLibrary.Conv_StringToText` (`KismetStringLibrary.Concat_StrStr` (`self.FirstName`) (`self.LastName`))) :!label _label))

(event `UpdateName`
  (goto _label))

(fn `UserConstructionScript`)