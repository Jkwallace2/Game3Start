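; Aggressive enemy Blueprint that configures a ranged, super-aggressive AI variant with self-preservation turned off.
; Its construction script sets inherited or member values for attack and strafe radii, behavior flags, health and a first and last name, then calls the parent construction script.
; The event graph holds only disabled default events, so this Blueprint adds no runtime logic of its own.
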(fn `UserConstructionScript`
  (set `self.Attack Radius` 800.0)
  (set `self.Strafe Radius` 1000.0)
  (set `self.AmIRangedEnemy` true)
  (set `self.SuperAgressive` true)
  (set `self.SelfPreservation` false)
  (set `self.Health` 200.0)
  (set `self.FirstName` "John")
  (set `self.LastName` "KYS")
  (`parent.UserConstructionScript`))