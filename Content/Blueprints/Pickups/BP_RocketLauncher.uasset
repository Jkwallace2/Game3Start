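; Rocket launcher weapon Blueprint that fires a rocket on primary use and a grenade on secondary use.
; Each shot plays a sound, waits briefly, then spawns the projectile ahead of the Sphere component along its facing.
; A shared Ammo boolean acts as a cooldown gate, restoring itself after a short delay.
; Either input during cooldown prints a reload message and plays a click.
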(event `self.ReceiveTick`
  (params (DeltaSeconds :type "Float (single-precision)"))
  (`parent.ReceiveTick` DeltaSeconds))

(event `self.UsePrimary`
  (bind _sphere (`self.Sphere`))
  (bind _returnvalue (`SceneComponent.K2_GetComponentLocation` (`self.Sphere`)))
  (if (`self.Ammo`)
    (set `self.Ammo` false)
    (`GameplayStatics.PlaySoundAtLocation` "/Game/Audio/ToyTank.ToyTank" _returnvalue (struct) 1.0 1.0 0.2 null null null null)
    (`KismetSystemLibrary.Delay` 0.3)
    (`|SpawnActorFromClass` "/Game/Blueprints/BP_Rocket.BP_Rocket_C" (`KismetMathLibrary.MakeTransform` (+ (`SceneComponent.K2_GetComponentLocation` _sphere) (* (`SceneComponent.GetForwardVector` _sphere) (200.0 200.0 200.0))) (`SceneComponent.K2_GetComponentRotation` _sphere)) "Undefined" "MultiplyWithRoot" null null)
    (`KismetSystemLibrary.Delay` 0.25 :!label _label)
    (set `self.Ammo` true)
    (else
      (`KismetSystemLibrary.PrintString` "RELOAD" true true (struct :`R` 1.0 :`B` 0.021873 :`A` 1.0) :!label _label_2)
      (`GameplayStatics.PlaySoundAtLocation` "/Game/Audio/ToyClick.ToyClick" _returnvalue (struct) 1.0 1.0 0.0 null null null null))))

(event `self.UseSecondary`
  (bind _sphere (`self.Sphere`))
  (if (`self.Ammo`)
    (set `self.Ammo` false)
    (`GameplayStatics.PlaySoundAtLocation` "/Game/Audio/ToyTank2.ToyTank2" (`SceneComponent.K2_GetComponentLocation` (`self.Sphere`)) (struct) 1.0 1.0 0.1 null null null null)
    (`KismetSystemLibrary.Delay` 0.3)
    (`|SpawnActorFromClass` "/Game/Blueprints/levelStuff/BP_Grenade.BP_Grenade_C" (`KismetMathLibrary.MakeTransform` (+ (`SceneComponent.K2_GetComponentLocation` _sphere) (* (`SceneComponent.GetForwardVector` _sphere) (200.0 200.0 200.0))) (`SceneComponent.K2_GetComponentRotation` _sphere)) "Undefined" "MultiplyWithRoot" null 3.0 2000.0 false null null)
    (goto _label)
    (else
      (goto _label_2))))

(fn `UserConstructionScript`
  (`parent.UserConstructionScript`))