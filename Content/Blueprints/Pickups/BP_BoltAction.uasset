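; Bolt-action toy rifle pickup that holds one chambered shot, fired with primary use and cycled with secondary use.
; Primary use clears the Ammo flag, plays a shot sound and line-traces forward from the Sphere, spawning a Niagara burst aligned to the impact normal, with no damage applied.
; Firing empty clicks and prints a reload message; secondary use then plays a slide sound, ejects brass and restores Ammo after a short delay.
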(event `self.ReceiveTick`
  (params (DeltaSeconds :type "Float (single-precision)"))
  (`parent.ReceiveTick` DeltaSeconds))

(event `self.UsePrimary`
  (bind _sphere (`self.Sphere`))
  (bind _returnvalue (`SceneComponent.K2_GetComponentLocation` _sphere))
  (bind _returnvalue_2 (`SceneComponent.K2_GetComponentLocation` (`self.Sphere`)))
  (bind _returnvalue_3 (`SceneComponent.GetForwardVector` _sphere))
  (if (`self.Ammo`)
    (set `self.Ammo` false)
    (`GameplayStatics.PlaySoundAtLocation` "/Game/Audio/ToyRifle.ToyRifle" _returnvalue_2 (struct) 1.0 1.0 0.25 null null null null)
    (bind (_outhit _returnvalue_4) (`KismetSystemLibrary.LineTraceSingle` (+ _returnvalue (* _returnvalue_3 60.0)) (+ _returnvalue (* _returnvalue_3 8000.0)) "TraceTypeQuery1"))
    (if _returnvalue_4
      (bind (_bblockinghit _binitialoverlap _time _distance _location _impactpoint _normal _impactnormal) (`GameplayStatics.BreakHitResult` _outhit))
      (`NiagaraFunctionLibrary.SpawnSystemAtLocation` "/Niagara/DefaultAssets/Templates/Systems/DirectionalBurst.DirectionalBurst" _location (`KismetMathLibrary.Conv_VectorToRotator` _impactnormal)))
    (else
      (`KismetSystemLibrary.PrintString` "RELOAD" true true (struct :`R` 1.0 :`B` 0.021873 :`A` 1.0))
      (`GameplayStatics.PlaySoundAtLocation` "/Game/Audio/ToyClick.ToyClick" _returnvalue_2 (struct) 1.0 1.0 0.0 null null null null))))

(event `self.UseSecondary`
  (bind _sphere (`self.Sphere`))
  (bind _returnvalue (`SceneComponent.GetForwardVector` _sphere))
  (if (not (`self.Ammo`))
    (`GameplayStatics.PlaySoundAtLocation` "/Game/Audio/ToySlide1.ToySlide1" (`SceneComponent.K2_GetComponentLocation` (`self.Sphere`)) (struct) 2.0 1.0 0.0 null null null null)
    (`NiagaraFunctionLibrary.SpawnSystemAtLocation` "/Game/VFX/NS_Brass.NS_Brass" (+ (`SceneComponent.K2_GetComponentLocation` _sphere) (* _returnvalue (40.0 40.0 50.0))) (`KismetMathLibrary.Conv_VectorToRotator` _returnvalue) (2.0 2.0 2.0))
    (`KismetSystemLibrary.Delay` 0.125)
    (set `self.Ammo` true)))

(fn `UserConstructionScript`
  (`parent.UserConstructionScript`))