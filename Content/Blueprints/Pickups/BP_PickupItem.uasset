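; Base-style pickup item actor that attaches to a skeletal mesh's right hand and can be dropped back into the world.
; Pickup plays a sound, prints a message, disables collision and snaps to the hand_r socket with a rotation offset.
; UpdateViewAngle turns the held item from the hand socket toward a look-at location.
; Drop fires the empty HasBeenDropped hook, detaches, restores collision and briefly simulates physics on the Sphere.
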(event `/Game/Blueprints/BPI_Item.Pickup`
  (params (SkeletalMesh :type "SkeletalMeshComponent Object Reference"))
  (`GameplayStatics.PlaySoundAtLocation` "/Game/Audio/ToySlide1.ToySlide1" (`self.K2_GetActorLocation`) (struct) 1.0 1.0 0.0 null null null null)
  (`KismetSystemLibrary.PrintText` (`|FormatText` "{name} is getting attached to {mesh}" (`KismetSystemLibrary.MakeLiteralString` (`KismetSystemLibrary.GetDisplayName` self)) SkeletalMesh))
  (`self.SetActorEnableCollision` false)
  (`self.K2_AttachToComponent` SkeletalMesh "hand_r" "SnapToTarget" "SnapToTarget" "SnapToTarget")
  (`self.K2_SetActorRelativeRotation` (`self.RotationOffset`)))

(event `/Game/Blueprints/BPI_Item.UpdateViewAngle`
  (params (LookAtLocation :type "Vector Structure"))
  (`self.K2_SetActorRotation` (`KismetMathLibrary.FindLookAtRotation` (`SceneComponent.GetSocketLocation` (stale `/Game/Blueprints/BPI_Item.Pickup` SkeletalMesh) "hand_r") LookAtLocation)))

(event `/Game/Blueprints/BPI_Item.Drop`
  (bind _sphere (`self.Sphere`))
  (`self.HasBeenDropped`)
  (`self.K2_DetachFromActor` "KeepWorld" "KeepWorld" "KeepWorld")
  (`self.SetActorEnableCollision` true)
  (`PrimitiveComponent.SetSimulatePhysics` _sphere true)
  (`KismetSystemLibrary.Delay` 2.0)
  (`PrimitiveComponent.SetSimulatePhysics` _sphere false))

(event `HasBeenDropped`)

(fn `UserConstructionScript`)