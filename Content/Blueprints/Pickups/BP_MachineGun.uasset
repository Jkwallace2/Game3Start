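; BP_MachineGun is a pickup weapon that fires automatically while primary use is held.
; UsePrimary loops on a short delay while IsDown is set, spawning a bullet, gunshot sound and Niagara brass effect from the Sphere component.
; UsePrimaryToggle sets IsDown and dropping the gun clears it.
; Secondary use toggles a laser, drawn each Tick purely as a line trace's one-frame debug line.
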(event `self.ReceiveTick`
  (params (DeltaSeconds :type "Float (single-precision)"))
  (bind _sphere (`self.Sphere`))
  (bind _returnvalue (`SceneComponent.K2_GetComponentLocation` _sphere))
  (bind _returnvalue_2 (`SceneComponent.GetForwardVector` _sphere))
  (`parent.ReceiveTick` DeltaSeconds)
  (if (`self.Lazer`)
    (`KismetSystemLibrary.LineTraceMulti` :`Start` (+ _returnvalue (* _returnvalue_2 60.0)) :`End` (+ _returnvalue (* _returnvalue_2 8000.0)) :`TraceChannel` "TraceTypeQuery1" :`DrawDebugType` "ForOneFrame")))

(event `/Game/Blueprints/BPI_Item.UsePrimary`
  (bind _sphere (`self.Sphere`))
  (bind _sphere_2 (`self.Sphere`))
  (bind _returnvalue (`SceneComponent.GetForwardVector` _sphere))
  (if (`self.IsDown`) :!label _label
    (`GameplayStatics.PlaySoundAtLocation` "/Game/Audio/ToyMachineGun2.ToyMachineGun2" (`SceneComponent.K2_GetComponentLocation` (`self.Sphere`)) (struct) 1.0 1.0 0.2 null null null null)
    (`|SpawnActorFromClass` "/Game/Blueprints/BP_Bullet.BP_Bullet_C" (`KismetMathLibrary.MakeTransform` (`SceneComponent.K2_GetComponentLocation` _sphere_2) (`SceneComponent.K2_GetComponentRotation` _sphere_2)) "Undefined" "MultiplyWithRoot" null null)
    (`NiagaraFunctionLibrary.SpawnSystemAtLocation` "/Game/VFX/NS_Brass.NS_Brass" (+ (`SceneComponent.K2_GetComponentLocation` _sphere) (* _returnvalue (40.0 40.0 50.0))) (`KismetMathLibrary.Conv_VectorToRotator` _returnvalue))
    (`KismetSystemLibrary.Delay` 0.1)
    (goto _label)))

(event `/Game/Blueprints/BPI_Item.UsePrimaryToggle`
  (params (IsDown :type Boolean))
  (set `self.IsDown` IsDown))

(event `self.HasBeenDropped`
  (set `self.IsDown` false))

(event `/Game/Blueprints/BPI_Item.UseSecondary`
  (bind _isa (`/Engine/EditorBlueprintResources/StandardMacros.FlipFlop`)
    (:`A`
      _)
    (:`B`
      _))
  (set `self.Lazer` _isa))

(fn `UserConstructionScript`
  (`parent.UserConstructionScript`))