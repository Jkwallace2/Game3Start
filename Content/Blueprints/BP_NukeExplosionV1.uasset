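; BP_NukeExplosionV1 is a nuke variant of an explosion actor, configured for a large damage radius and high damage.
; It has no active event logic of its own, as the BeginPlay, overlap and Tick events are disabled stubs.
; The construction script calls the parent's, then sets damage, radius, the NS_Nuke effect template, and sound volume and lowered pitch.
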(fn `UserConstructionScript`
  (`parent.UserConstructionScript`)
  (set `self.DamageRadius` 4000.0)
  (set `self.Damage` 500.0)
  (set `self.System Template` "/Game/VFX/NS_Nuke.NS_Nuke")
  (set `self.Volume` 2.0)
  (set `self.Pitch` 0.6))