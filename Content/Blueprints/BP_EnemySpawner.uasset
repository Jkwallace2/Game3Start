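; Enemy spawner that populates the level with randomized, named BP_AiMoveTo enemies on BeginPlay.
; Each BP_EnemySpawnPoint actor has a weighted chance to spawn one enemy at its transform.
; A counter walks the shuffled first-name list for unique first names, skipping index zero and lacking overflow handling.
; Last names, skeletal meshes and materials are picked randomly and may repeat, and the combined name feeds the enemy's name text.
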(event `self.ReceiveBeginPlay`
  (set `self.Namebus` 0)
  ; Shuffle First names
  (`KismetArrayLibrary.Array_Shuffle` (`self.FirstNames`))
  (`KismetSystemLibrary.PrintString` "EnemySpawnerIsActive")
  (bind _outactors (`GameplayStatics.GetAllActorsOfClass` "/Game/Blueprints/BP_EnemySpawnPoint.BP_EnemySpawnPoint_C"))
  (for _array_element _outactors
    (if (`KismetMathLibrary.RandomBoolWithWeight` 0.75)
      ; make sure we only take a name card if the enemy exists
      (`/Engine/EditorBlueprintResources/StandardMacros.IncrementInt` (`self.Namebus`)
        (:`  `
          (bind _returnvalue (`|SpawnActorFromClass` "/Game/AI_Blueprints/BP_AiMoveTo.BP_AiMoveTo_C" (`self.GetTransform` _array_element) "Undefined" "MultiplyWithRoot" null null))
          ; unique first names, one of each, no implementation of overflow
          (bind _output_get (set `/Game/AI_Blueprints/BP_AiMoveTo.FirstName` (`|GetArrayItem` (`self.FirstNames`) (`self.Namebus`)) _returnvalue))
          ; Random last name, npcs may share last name
          (bind _output_get_2 (set `/Game/AI_Blueprints/BP_AiMoveTo.LastName` (`KismetArrayLibrary.Array_Random` (`self.LastNames`)) _returnvalue))
          (`TextRenderComponent.K2_SetText` (`/Game/AI_Blueprints/BP_AiMoveTo.AI FirstName` _returnvalue) (`KismetTextLibrary.Conv_StringToText` (`KismetStringLibrary.Concat_StrStr` _output_get " " _output_get_2)))
          (bind _mesh (`Character.Mesh` _returnvalue))
          (`SkeletalMeshComponent.SetSkeletalMeshAsset` _mesh (`KismetArrayLibrary.Array_Random` (`self.MeshList`)))
          (`PrimitiveComponent.SetMaterial` _mesh 0 (`KismetArrayLibrary.Array_Random` (`self.Materials`)))))
      (else
        (`KismetSystemLibrary.PrintString` "Enemy denied existance")))))

(fn `UserConstructionScript`)