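; BP_Grenade is a bouncing projectile grenade that explodes on a short timed fuse.
; BeginPlay waits out the fuse, spawns BP_Explosion at the grenade's location, then destroys the grenade shortly after.
; ProjectileMovement bounces, capped by countdown I, emit noise and a sound at the impact point.
; On valid hits they also call ApplyDamage credited to player controller 0, though no damaged actor is wired in.
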(event `self.ReceiveTick`
  (params (DeltaSeconds :type "Float (single-precision)")))

(event `self.ReceiveBeginPlay`
  (`KismetSystemLibrary.Delay` 2.0)
  (`|SpawnActorFromClass` "/Game/Blueprints/BP_Explosion.BP_Explosion_C" (`KismetMathLibrary.Conv_VectorToTransform` (`self.K2_GetActorLocation`)) "Undefined" "MultiplyWithRoot" null self (`self.GetInstigator`))
  (`KismetSystemLibrary.Delay` 0.1)
  (`self.K2_DestroyActor`))

(event `self.ProjectileMovement.OnProjectileBounce`
  (params (ImpactResult :type "HitResult Structure (by ref)") (ImpactVelocity :type "Vector Structure (by ref)"))
  (if (> (`self.i`) 0)
    (`/Engine/EditorBlueprintResources/StandardMacros.DecrementInt` (`self.i`)
      (:`  `
        (`self.MakeNoise` 3.0 (`self.GetInstigator`) ImpactResult_Location)
        (`GameplayStatics.PlaySoundAtLocation` "/Game/Audio/bubble2.bubble2" ImpactResult_Location (struct) 1.0 1.0 0.0 null null null null)
        (`/Engine/EditorBlueprintResources/StandardMacros.IsValid` ImpactResult_HitActor
          (:`Is Valid`
            (`GameplayStatics.ApplyDamage` null 1.0 (`GameplayStatics.GetPlayerController` 0) self)))))))

(fn `UserConstructionScript`)