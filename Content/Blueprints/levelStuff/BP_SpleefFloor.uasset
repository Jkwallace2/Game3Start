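; BP_SpleefFloor is a breakable floor block, named for spleef, that wears down under point damage.
; Each hit subtracts scaled damage from Health and swaps the mesh material to a damage stage derived from the remaining Health.
; At zero Health it spawns a block-break Niagara effect oriented to the hit normal and destroys itself.
; A very large hit skips this, spawning an explosion and destroying the block a tick later.
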(event `self.ReceivePointDamage`
  (params (Damage :type "Float (single-precision)") (DamageType :type "DamageType Object Reference") (HitLocation :type "Vector Structure") (HitNormal :type "Vector Structure") (HitComponent :type "PrimitiveComponent Object Reference") (BoneName :type Name) (ShotFromDirection :type "Vector Structure") (InstigatedBy :type "Controller Object Reference") (DamageCauser :type "Actor Object Reference") (HitInfo :type "HitResult Structure (by ref)"))
  (if (> Damage 800.0)
    (`NiagaraFunctionLibrary.SpawnSystemAtLocation` "/Game/VFX/NS_ExplosionSimple.NS_ExplosionSimple" (`self.K2_GetActorLocation`))
    (`KismetSystemLibrary.DelayUntilNextTick`)
    (`self.K2_DestroyActor`)
    (else
      (bind _output_get (set `self.Health` (- (`self.Health`) (* Damage 0.2))))
      (`self.UpdateMaterial`)
      (if (<= _output_get 0)
        (`NiagaraFunctionLibrary.SpawnSystemAtLocation` "/Game/VFX/NS_BlockBreak.NS_BlockBreak" HitLocation (`KismetMathLibrary.Conv_VectorToRotator` HitNormal))
        (`self.K2_DestroyActor`)))))

(event `self.ReceiveAnyDamage`
  (params (Damage :type "Float (single-precision)") (DamageType :type "DamageType Object Reference") (InstigatedBy :type "Controller Object Reference") (DamageCauser :type "Actor Object Reference")))

(event `UpdateMaterial`
  (bind _staticmesh (`self.StaticMesh`))
  (switch `int` (- 6 (`self.Health`))
    (:`0`
      (`PrimitiveComponent.SetMaterial` _staticmesh 0 "/Game/Blueprints/levelStuff/MI_Bamage0.MI_Bamage0"))
    (:`1`
      (`PrimitiveComponent.SetMaterial` _staticmesh 0 "/Game/Blueprints/levelStuff/MI_Bamage1.MI_Bamage1"))
    (:`2`
      (`PrimitiveComponent.SetMaterial` _staticmesh 0 "/Game/Blueprints/levelStuff/MI_Bamage2.MI_Bamage2"))
    (:`3`
      (`PrimitiveComponent.SetMaterial` _staticmesh 0 "/Game/Blueprints/levelStuff/MI_Bamage3.MI_Bamage3"))
    (:`4`
      (`PrimitiveComponent.SetMaterial` _staticmesh 0 "/Game/Blueprints/levelStuff/MI_Bamage4.MI_Bamage4"))
    (:`5`
      (`PrimitiveComponent.SetMaterial` _staticmesh 0 "/Game/Blueprints/levelStuff/MI_Bamage5.MI_Bamage5"))))

(fn `UserConstructionScript`)