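; BP_Grenade is a timed bomb thrown as an optionally homing projectile, or spawned idle as a physics object.
; A Delay in Tick steps the fuse every 0.1 seconds, driving material, ticking sound and AI noise until it spawns BP_Explosion.
; Bounces detonate it against other grenades or bomb-holding characters, otherwise making noise and applying speed-based impact damage and knockback.
; Idle grenades carry gameplay Risk tags keyed to fuse level.
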(event `self.ReceiveTick`
  (params (DeltaSeconds :type "Float (single-precision)"))
  (bind _returnvalue (`KismetMathLibrary.MapRangeClamped` (`KismetMathLibrary.Conv_IntToDouble` (`self.LitFuse`)) 0.0 29.0 1.0))
  ; Fuse
  ;; "is Fuse Lit"
  (if (`self.SpawnIdle`)
    (`self.No longer safe`)
    (else
      (`KismetSystemLibrary.Delay` 0.1)
      (bind _result (`/Engine/EditorBlueprintResources/StandardMacros.DecrementInt` (`self.LitFuse`))
        (:`  `
          (`MeshComponent.SetScalarParameterValueOnMaterials` (`self.Sphere1`) "Fuse" _returnvalue)
          (if (== (mod _result 4) 0)
            (bind _returnvalue_2 (`GameplayStatics.SpawnSoundAttached` "/Game/Audio/SC_TickingBomb.SC_TickingBomb" (`self.Sphere`) "None" (0.0 0.0 0.0) (struct) "KeepRelativeOffset" false 1.0 1.0 0.0 null null))
            (`AudioParameterControllerInterface.SetFloatParameter` _returnvalue_2 "Blend" _returnvalue)
            (if (<= (`self.LitFuse`) 15)
              (`self.MakeNoise` 1.0 (`GameplayStatics.GetPlayerPawn` 0) (`SceneComponent.K2_GetComponentLocation` (`self.Sphere`)))))
          (if (<= (`self.LitFuse`) 0)
            (`self.Splode`)))))))

(event `No longer safe`
  (bind _tag_container (`self.Tag Container`))
  (if (<= (`self.LitFuse`) 5)
    (`/Engine/EditorBlueprintResources/StandardMacros.DoOnce` false
      (:`Completed`
        (`BlueprintGameplayTagLibrary.RemoveGameplayTag` _tag_container (struct :`TagName` "Risk.High"))
        (`BlueprintGameplayTagLibrary.AddGameplayTag` _tag_container (struct :`TagName` "Risk.Severe"))))
    (elif (<= (`self.LitFuse`) 15)
      (`/Engine/EditorBlueprintResources/StandardMacros.DoOnce` false
        (:`Completed`
          (`BlueprintGameplayTagLibrary.RemoveGameplayTag` _tag_container (struct :`TagName` "Risk.Medium"))
          (`BlueprintGameplayTagLibrary.AddGameplayTag` _tag_container (struct :`TagName` "Risk.High"))))
      (elif (<= (`self.LitFuse`) 25)
        (`/Engine/EditorBlueprintResources/StandardMacros.DoOnce` false
          (:`Completed`
            (`BlueprintGameplayTagLibrary.RemoveGameplayTag` _tag_container (struct :`TagName` "Risk.Low"))
            (`BlueprintGameplayTagLibrary.AddGameplayTag` _tag_container (struct :`TagName` "Risk.Medium"))))))))

(event `Splode`
  (`|SpawnActorFromClass` "/Game/Blueprints/BP_Explosion.BP_Explosion_C" (`KismetMathLibrary.Conv_VectorToTransform` (`self.K2_GetActorLocation`)) "Undefined" "MultiplyWithRoot" null self (`self.GetInstigator`))
  (`self.K2_DestroyActor`))

(event `self.ReceiveBeginPlay`
  (bind _homingtarget (`self.HomingTarget`))
  (bind _projectilemovement (`self.ProjectileMovement`))
  (bind _initialspeed (`self.initialSpeed`))
  (`GameplayStatics.SpawnSoundAttached` "/Game/Audio/SC_BallThrow.SC_BallThrow" (`self.Sphere`) "None" (0.0 0.0 0.0) (struct) "KeepRelativeOffset" false 1.0 1.0 0.0 null null)
  (if (`self.SpawnIdle`)
    (`PrimitiveComponent.SetSimulatePhysics` (`self.Sphere`) true)
    (set `self.LitFuse` 30)
    (`BlueprintGameplayTagLibrary.AddGameplayTag` (`self.Tag Container`) (struct :`TagName` "Risk.Medium"))
    (else
      (if (`KismetSystemLibrary.IsValid` _homingtarget)
        (set `ProjectileMovementComponent.HomingTargetComponent` (`self.GetParentComponent` _homingtarget) (`self.ProjectileMovement`))
        (else
          (set `ProjectileMovementComponent.bIsHomingProjectile` false (`self.ProjectileMovement`))))
      (`PrimitiveComponent.SetSimulatePhysics` (`self.Sphere`) false)
      (bind _output_get (set `ProjectileMovementComponent.InitialSpeed` _initialspeed _projectilemovement))
      ; For Homing
      (set `ProjectileMovementComponent.MaxSpeed` _initialspeed _projectilemovement)
      (`ProjectileMovementComponent.SetVelocityInLocalSpace` (`self.ProjectileMovement`) (`KismetMathLibrary.MakeVector` _output_get))
      (set `self.LitFuse` (+ (`KismetMathLibrary.FTrunc` (* (`self.Fuse`) 10.0)) 1)))))

(event `self.ProjectileMovement.OnProjectileBounce`
  (params (ImpactResult :type "HitResult Structure (by ref)") (ImpactVelocity :type "Vector Structure (by ref)"))
  (bind _returnvalue (`GameplayStatics.GetPlayerPawn` 0))
  (bind _returnvalue_2 (`KismetMathLibrary.VSize` ImpactVelocity))
  (bind (_bblockinghit _binitialoverlap _time _distance _location _impactpoint _normal _impactnormal _physmat _hitactor _hitcomponent) (`GameplayStatics.BreakHitResult` ImpactResult))
  (bind _returnvalue_3 (> (`self.i`) 4))
  (bind _returnvalue_4 (* _normal (* _returnvalue_2 -1.0)))
  ; Splode when hitting other bombs
  (bind _asbp_grenade (cast `/Game/Blueprints/levelStuff/BP_Grenade` _hitactor)
    (:`then`
      (`self.Splode`))
    (:`CastFailed`
      (bind _asbp_enemy_base (cast `/Game/AI_Blueprints/BP_EnemyBase` _hitactor)
        (:`then`
          (if (`/Game/AI_Blueprints/BP_EnemyBase.IsHoldingBomb` _asbp_enemy_base)
            (`self.Splode`)
            (else
              (bind _asbp_state_tree_player (cast `/Game/DoubleAction/FirstPerson/Blueprints/BP_StateTreePlayer` _hitactor :!label _label)
                (:`then`
                  (if (`/Game/DoubleAction/FirstPerson/Blueprints/BP_StateTreePlayer.IsHoldingBomb` _asbp_state_tree_player)
                    (`self.Splode`)
                    (else
                      (if (> (`self.i`) 0) :!label _label_2
                        (`/Engine/EditorBlueprintResources/StandardMacros.DecrementInt` (`self.i`)
                          (:`  `
                            (if (> _returnvalue_2 5500.0)
                              (`self.MakeNoise` 3.0 _returnvalue)
                              (`GameplayStatics.SpawnSoundAttached` "/Game/Audio/ViolentDodgeBall_Cue.ViolentDodgeBall_Cue" _hitcomponent "None" (0.0 0.0 0.0) (struct) "SnapToTarget" false 1.0 1.0 0.0 null null)
                              (if _returnvalue_3
                                (set `self.knock` (* _returnvalue_4 2.0))
                                (set `self.Damage` 200.0)
                                (`/Engine/EditorBlueprintResources/StandardMacros.IsValid` _hitactor :!label _label_3
                                  (:`Is Valid`
                                    (bind _ascharacter (cast `Character` _hitactor)
                                      (:`then`
                                        (`CharacterMovementComponent.AddImpulse` (`Character.CharacterMovement` _ascharacter) (`self.knock`) true))
                                      (:`CastFailed`
                                        _))
                                    (`GameplayStatics.ApplyPointDamage` _hitactor (`self.Damage`) _impactpoint ImpactResult))))
                              (else
                                (`self.MakeNoise` 1.0 _returnvalue _impactpoint)
                                (`GameplayStatics.SpawnSoundAttached` "/Game/Audio/CopyInfDodgeball_Cue.CopyInfDodgeball_Cue" (`self.Sphere1`) "None" (0.0 0.0 0.0) (struct) "SnapToTarget" false (`KismetMathLibrary.MapRangeClamped` _returnvalue_2 1.0 4000.0 0.01 1.0) 1.0 0.0 null null)
                                (if _returnvalue_3
                                  (set `self.knock` (* _returnvalue_4 0.25))
                                  (set `self.Damage` 10.0)
                                  (goto _label_3))))))))))
                (:`CastFailed`
                  (goto _label_2))))))
        (:`CastFailed`
          (goto _label))))))

(fn `UserConstructionScript`
  (if (`self.SpawnIdle`)
    (`BlueprintGameplayTagLibrary.AddGameplayTag` (`self.Tag Container`) (struct :`TagName` "Risk.Low"))))

(fn `WhachaFuseAt`
  (returns (CeilFuse :type Integer))
  (return (`self.LitFuse`)))