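; Wave-based trigger that runs up to three rounds of activations and fires once its box is clear of enemies.
; PreTrigger messages the Round1 actors, opens a gate after a short delay and slows Tick to half-second polling.
; When no BP_EnemyBase overlaps the box, Tick decrements Rounds, then either activates Round2 or Round3 (falling back to Round2 if empty) or calls Trigger at zero.
; It also prints the enemy count for debugging.
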(event `self.ReceiveTick`
  (params (DeltaSeconds :type "Float (single-precision)"))
  (bind _round3 (`self.Round3`))
  (bind _rounds (`self.Rounds`))
  (bind _returnvalue (`KismetArrayLibrary.Array_Length` (`PrimitiveComponent.GetOverlappingActors` (`self.Box`) "/Game/AI_Blueprints/BP_EnemyBase.BP_EnemyBase_C")))
  (`parent.ReceiveTick` DeltaSeconds)
  (if (`self.Gate`)
    (`KismetSystemLibrary.PrintString` (`KismetStringLibrary.Conv_IntToString` _returnvalue))
    (if (<= _returnvalue 0)
      (`/Engine/EditorBlueprintResources/StandardMacros.DecrementInt` _rounds
        (:`  `
          (if (<= _rounds 0)
            (`self.Trigger`)
            (elif (== (`self.Rounds`) 2)
              (set `self.Gate` false)
              (for _array_element (`self.Round2`) :!label _label
                (message `/Game/Blueprints/BPI_InWorldCommunication.Activate` _array_element)
                (`KismetSystemLibrary.Delay` 1.0)
                (set `self.Gate` true))
              (elif (== (`self.Rounds`) 1)
                (set `self.Gate` false)
                (if (> (`KismetArrayLibrary.Array_Length` _round3) 0)
                  (for _array_element_2 _round3
                    (message `/Game/Blueprints/BPI_InWorldCommunication.Activate` _array_element_2)
                    (`KismetSystemLibrary.Delay` 1.0)
                    (set `self.Gate` true))
                  (else
                    (goto _label)))))))))))

(event `self.Pre Trigger`
  (for _array_element (`self.Round1`)
    (message `/Game/Blueprints/BPI_InWorldCommunication.Activate` _array_element))
  (`KismetSystemLibrary.Delay` 1.0)
  (set `self.Gate` true)
  (`self.SetActorTickInterval` 0.5))

(fn `UserConstructionScript`
  (`parent.UserConstructionScript`))