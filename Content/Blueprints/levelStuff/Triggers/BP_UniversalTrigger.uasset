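; Universal trigger volume that activates and deactivates lists of other objects when the player pawn enters its box while it is active.
; An Activate event arms it, and a valid overlap runs PreTrigger, a hook for children to override that calls Trigger by default.
; Trigger prints a debug string, messages both object lists, and destroys the actor if DoOnce is set.
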(event `/Game/Blueprints/BPI_InWorldCommunication.Activate`
  (set `self.IsActive` true))

(event `self.Box.OnComponentBeginOverlap`
  (params (OverlappedComponent :type "PrimitiveComponent Object Reference") (OtherActor :type "Actor Object Reference") (OtherComp :type "PrimitiveComponent Object Reference") (OtherBodyIndex :type Integer) (bFromSweep :type Boolean) (SweepResult :type "HitResult Structure (by ref)"))
  (if (`self.IsActive`)
    (if (== OtherActor (`GameplayStatics.GetPlayerPawn` 0))
      (if (`self.DoOnce?`)
        (`/Engine/EditorBlueprintResources/StandardMacros.DoOnce` false
          (:`Completed`
            _)))
      (`self.Pre Trigger`))))

(event `Trigger`
  (`KismetSystemLibrary.PrintString` "Universal Trigger" true true (struct :`R` 0.971012 :`G` 1.0 :`A` 1.0))
  (for _array_element (`self.ObjectsToActivate`)
    (message `/Game/Blueprints/BPI_InWorldCommunication.Activate` _array_element))
  (for _array_element_2 (`self.ObjectsToDeactivate`)
    (message `/Game/Blueprints/BPI_InWorldCommunication.Deactivate` _array_element_2))
  (if (`self.DoOnce?`)
    (`self.K2_DestroyActor`)))

(event `Pre Trigger`
  ; Let children overide
  (`self.Trigger`))

(fn `UserConstructionScript`)