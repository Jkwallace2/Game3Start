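; BP_NormalDoor is a door that slides down to open once activated and has no logic to close again.
; Activate runs only once, registers the door in the GM_SavLod game mode's OpenedNormalDoors level state, and plays a Timeline that lerps the Door component's relative height.
; Softopen snaps the door straight to the open position and sets the opened flag, skipping both animation and registration.
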(event `Soft open`
  (set `self.IsAlredyOpened` true)
  (`SceneComponent.K2_SetRelativeLocation` (`self.Door`) (0.0 0.0 -130.0) false false))

(event `/Game/Blueprints/BPI_InWorldCommunication.Activate`
  (if (not (`self.IsAlredyOpened`))
    (set `self.IsAlredyOpened` true)
    (bind _asgm_sav_lod (cast `/Game/Blueprints/SavingAndLoading/GM_SavLod` (`GameplayStatics.GetGameMode`))
      (:`then`
        (`KismetArrayLibrary.Array_AddUnique` (`/Game/Blueprints/SavingAndLoading/SG_LevelState.OpenedNormalDoors` (`/Game/Blueprints/SavingAndLoading/GM_SavLod.SG_LevelState` _asgm_sav_lod)) self)
        (bind (_direction _newtrack_0) (`Timeline|Timeline` :!label _label)
          (:`Update`
            (`SceneComponent.K2_SetRelativeLocation` (`self.Door`) (`KismetMathLibrary.VLerp` (0.0 0.0 150.0) (0.0 0.0 -130.0) _newtrack_0) false false))))
      (:`CastFailed`
        (goto _label)))))

(fn `UserConstructionScript`)