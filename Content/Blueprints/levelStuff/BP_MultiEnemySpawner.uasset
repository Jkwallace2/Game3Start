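; BP_MultiEnemySpawner is an activatable spawner that creates a series of actors of a configurable class at its Billboard's transform.
; Activate waits out a warm-up, then runs a delayed countdown loop that spawns one actor per step until the configured count is used up.
; A DoOnce flag marks the spawner as single-use, destroying it when the series finishes.
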(event `/Game/Blueprints/BPI_InWorldCommunication.Activate`
  (`KismetSystemLibrary.Delay` (`self.WarmUp`))
  (if (`self.DoOnce`)
    (`/Engine/EditorBlueprintResources/StandardMacros.DoOnce` false
      (:`Completed`
        _)))
  (set `self.I` (`self.Count`))
  (if (> (`self.I`) 0) :!label _label
    (`/Engine/EditorBlueprintResources/StandardMacros.DecrementInt` (`self.I`)
      (:`  `
        (`|SpawnActorFromClass` (`self.Class`) (`SceneComponent.K2_GetComponentToWorld` (`self.Billboard`)) "Undefined" "MultiplyWithRoot" null null)
        (`KismetSystemLibrary.Delay` (`self.Delay`))
        (goto _label)))
    (elif (`self.DoOnce`)
      (`self.K2_DestroyActor`))))

(fn `UserConstructionScript`)