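; Machine gun pickup actor built from cube components, with events for being picked up, dropped and used.
; Pickup snaps it to the hand_r socket of the given skeletal mesh and disables collision on all three cubes.
; Drop detaches it, re-enables collision on the main cube only and simulates physics on that cube for a short delay.
; Primary use only prints a debug message, with no firing logic.
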(event `self.ReceiveBeginPlay`
  (`KismetSystemLibrary.PrintString` "Hello"))

(event `/Game/Blueprints/BPI_Item.Pickup`
  (params (SkeletalMesh :type "SkeletalMeshComponent Object Reference"))
  (`KismetSystemLibrary.PrintText` (`|FormatText` "{name} is getting attached to {mesh}" "machine gun" SkeletalMesh))
  (`self.K2_AttachToComponent` SkeletalMesh "hand_r" "SnapToTarget" "SnapToTarget" "SnapToTarget")
  (`PrimitiveComponent.SetCollisionEnabled` (`self.Cube`) "NoCollision")
  (`PrimitiveComponent.SetCollisionEnabled` (`self.Cube1`) "NoCollision")
  (`PrimitiveComponent.SetCollisionEnabled` (`self.Cube2`) "NoCollision"))

(event `/Game/Blueprints/BPI_Item.Drop`
  (bind _cube (`self.Cube`))
  (`self.K2_DetachFromActor` "KeepWorld" "KeepWorld" "KeepWorld")
  (`PrimitiveComponent.SetSimulatePhysics` _cube true)
  (`PrimitiveComponent.SetCollisionEnabled` _cube "QueryAndPhysics")
  (`KismetSystemLibrary.Delay` 2.0)
  (`PrimitiveComponent.SetSimulatePhysics` (`self.Cube`) false))

(event `/Game/Blueprints/BPI_Item.UsePrimary`
  (`KismetSystemLibrary.PrintString` "i am used" true true (struct :`R` 1.0 :`G` 0.784908 :`A` 1.0)))

(fn `UserConstructionScript`)