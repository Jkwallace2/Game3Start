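; BP_ElementalBarrier is a barrier actor that ends the game when a player character without matching elemental immunity touches it.
; On BeginPlay it writes its ElementalType to a TextRender label, followed by a switch on that type with no actions attached.
; Cube overlap compares BP_ThirdPersonCharacter's ElementalImmunity to the barrier's type; on a mismatch it prints a death message and quits the game after a short delay.
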(event `self.ReceiveBeginPlay`
  (`TextRenderComponent.K2_SetText` (`self.TextRender`) (`|GenericToText` (`self.ElementalType`)))
  (switch `/Game/Blueprints/ElementalType` (`self.ElementalType`)))

(event `self.Cube.OnComponentBeginOverlap`
  (params (OverlappedComponent :type "PrimitiveComponent Object Reference") (OtherActor :type "Actor Object Reference") (OtherComp :type "PrimitiveComponent Object Reference") (OtherBodyIndex :type Integer) (bFromSweep :type Boolean) (SweepResult :type "HitResult Structure (by ref)"))
  (bind _asbp_third_person_character (cast `/Game/ThirdPerson/Blueprints/BP_ThirdPersonCharacter` OtherActor))
  (if (not (`|EnumEquality` (`/Game/ThirdPerson/Blueprints/BP_ThirdPersonCharacter.ElementalImmunity` _asbp_third_person_character) (`self.ElementalType`)))
    (`KismetSystemLibrary.PrintString` "you ded")
    (`KismetSystemLibrary.Delay` 0.2)
    (`KismetSystemLibrary.QuitGame` null "Quit")))

(fn `UserConstructionScript`)