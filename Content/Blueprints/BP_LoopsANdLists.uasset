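; BP_LoopsANdLists is a Blueprint that demonstrates loops and arrays through on-screen debug printing.
; BeginPlay fills ColorArray with fixed colors and starts DelayLoop, an endless loop made by wiring execution back to its start through a half-second Delay.
; Each pass prints and increments LoopCount, then PrintColors shuffles the array and prints every index as text in that element's color.
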(event `self.ReceiveBeginPlay`
  (set `self.ColorArray` (`|MakeArray` (struct :`R` 1.0 :`G` 0.12722 :`B` 0.056962 :`A` 1.0) (struct :`R` 1.0 :`G` 0.814601 :`B` 0.032862 :`A` 1.0) (struct :`R` 0.451731 :`G` 1.0 :`B` 0.225254 :`A` 1.0) (struct :`R` 0.01948 :`G` 1.0 :`B` 0.403199 :`A` 1.0) (struct :`R` 0.397183 :`G` 0.370693 :`B` 1.0 :`A` 1.0) (struct :`R` 0.292077 :`G` 0.929617 :`B` 1.0 :`A` 1.0) (struct :`R` 0.439794 :`G` 0.21436 :`B` 1.0 :`A` 1.0) (struct :`R` 1.0 :`G` 0.019958 :`B` 0.964711 :`A` 1.0) (struct :`R` 1.0 :`B` 0.135831 :`A` 1.0) :!type "LinearColor Structure"))
  (`KismetSystemLibrary.PrintString` "LandL Active")
  (`self.Delay loop`))

(event `Delay loop`
  (bind _loopcount (`self.LoopCount`))
  (`KismetSystemLibrary.PrintString` (`KismetStringLibrary.Concat_StrStr` "loop" (`KismetStringLibrary.Conv_IntToString` _loopcount)) :!label _label)
  (`/Engine/EditorBlueprintResources/StandardMacros.IncrementInt` _loopcount
    (:`  `
      (`KismetSystemLibrary.Delay` 0.5)
      (`self.PrintColors`)
      (goto _label))))

(event `PrintColors`
  (`KismetArrayLibrary.Array_Shuffle` (`self.ColorArray`))
  (for (_array_element _array_index) (`self.ColorArray`)
    (`KismetSystemLibrary.PrintString` (`KismetStringLibrary.Concat_StrStr` "Colors " (`KismetStringLibrary.Conv_IntToString` _array_index)) true true _array_element)))

(fn `UserConstructionScript`)