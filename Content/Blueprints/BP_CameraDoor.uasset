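; BP_CameraDoor is a one-time door that shows itself opening through a camera cut.
; OpenDoor records the door in GM_SavLod's level state, blends the view to itself, then lowers the Door component with a timeline.
; After a two-second hold, the camera blends back to the supplied view target in half the time.
; Softopen snaps the door to its open position without camera or animation and marks it opened.
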(event `Soft open`
  (set `self.IsAlredyOpened` true)
  (`SceneComponent.K2_SetRelativeLocation` (`self.Door`) (0.0 0.0 -155.0) false false))

(event `OpenDoor`
  (params (NewViewTarget :type "Actor Object Reference"))
  (if (not (`self.IsAlredyOpened`))
    (set `self.IsAlredyOpened` true)
    (bind _asgm_sav_lod (cast `/Game/Blueprints/SavingAndLoading/GM_SavLod` (`GameplayStatics.GetGameMode`))
      (:`then`
        (`KismetArrayLibrary.Array_AddUnique` (`/Game/Blueprints/SavingAndLoading/SG_LevelState.OpenedDoors` (`/Game/Blueprints/SavingAndLoading/GM_SavLod.SG_LevelState` _asgm_sav_lod)) self))
      (:`CastFailed`
        _))
    (`PlayerController.SetViewTargetWithBlend` (`GameplayStatics.GetPlayerController` 0) self (`self.Blend Time`) "VTBlend_Cubic" 0.0 true)
    (`KismetSystemLibrary.Delay` (`self.Blend Time`))
    (bind (_direction _newtrack_0) (`Timeline|Timeline`)
      (:`Update`
        (`SceneComponent.K2_SetRelativeLocation` (`self.Door`) (`KismetMathLibrary.VLerp` (0.0 0.0 150.0) (0.0 0.0 -155.0) _newtrack_0) false false))
      (:`Finished`
        (`KismetSystemLibrary.Delay` 2.0) ; waiting 2 seconds while the door opens
        (`PlayerController.SetViewTargetWithBlend` (`GameplayStatics.GetPlayerController` 0) NewViewTarget (/ (`self.Blend Time`) 2.0) "VTBlend_Cubic" 0.0 false) ; shift camera back to player
      ))))

(fn `UserConstructionScript`)