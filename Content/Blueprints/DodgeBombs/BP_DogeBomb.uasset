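; The player's held bomb in a dodge-bomb game, handling catching, cooking and throwing.
; Catching sphere-overlaps BP_Grenades ahead of the camera and requests pickup; Transfer grants health, sets type and mesh, and carries over the fuse.
; Lit bombs count down through a Delay on Tick, driving material and ticking-sound feedback, and explode if still held at zero.
; Throwing spawns a BP_Grenade with the remaining fuse, charge-scaled speed and homing target.
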(event `self.ReceiveBeginPlay`
  (`parent.ReceiveBeginPlay`)
  (`self.LoseBomb`))

(event `EnhancedInput|/Game/DoubleAction/FirstPerson/Input/Actions/IA_cook`
  (params (ActionValue :type Boolean) (ElapsedSeconds :type "Float (double-precision)") (TriggeredSeconds :type "Float (double-precision)") (InputAction :type "InputAction Object Reference" :default "/Game/DoubleAction/FirstPerson/Input/Actions/IA_cook.IA_cook"))
  (:`Started`
    (if (`self.HasBomb`)
      (`self.cookBomb`)
      (else
        (`self.Try To catch Bomb`)))))

(event `cookBomb`
  ; CookingBomb
  (set `self.isLit` true)
  (`GameplayStatics.PlaySound2D` "/Engine/VREditor/Sounds/UI/Floating_UI_Close.Floating_UI_Close" 1.0 1.0 0.0 null null)
  (`/Engine/EditorBlueprintResources/StandardMacros.DoOnce` false :!label _label
    (:`Completed`
      (`/Game/DoubleAction/FirstPerson/Blueprints/BP_StateTreePlayer.StartThrowTimer` (`self.As BP State Tree Player`)))))

(event `EnhancedInput|/Game/DoubleAction/FirstPerson/Input/Actions/IA_Throw`
  (params (ActionValue :type Boolean) (ElapsedSeconds :type "Float (double-precision)") (TriggeredSeconds :type "Float (double-precision)") (InputAction :type "InputAction Object Reference" :default "/Game/DoubleAction/FirstPerson/Input/Actions/IA_Throw.IA_Throw"))
  (bind _firstpersoncamera (`/Game/DoubleAction/FirstPerson/Blueprints/BP_StateTreePlayer.FirstPersonCamera` (`self.As BP State Tree Player`)))
  (:`Completed`
    (`|ExecutionSequence`
      (:`then_0`
        (if (`self.HasBomb`)
          (`|SpawnActorFromClass` "/Game/Blueprints/DodgeBombs/BP_Grenade.BP_Grenade_C" (`KismetMathLibrary.MakeTransform` (+ (`SceneComponent.K2_GetComponentLocation` _firstpersoncamera) (* (`SceneComponent.GetForwardVector` _firstpersoncamera) 50.0)) (`SceneComponent.K2_GetComponentRotation` _firstpersoncamera)) "Undefined" "MultiplyWithRoot" null (* (`KismetMathLibrary.Conv_IntToDouble` (- (`self.InFuse`) 1)) 0.1) (`KismetMathLibrary.Lerp` 2000.0 8000.0 (`self.ThrowPower`)) false (`/Game/DoubleAction/FirstPerson/Blueprints/BP_StateTreePlayer.HomingActor` (`self.As BP State Tree Player`)) (`self.BombToThrow`) (`GameplayStatics.GetPlayerPawn` 0) null)
          (`self.LoseBomb`)))
      (:`then_1`
        (goto _label :!via `Reset`))
      (:`then_2`
        (`/Game/DoubleAction/FirstPerson/Blueprints/BP_StateTreePlayer.StopThrowTimer` (`self.As BP State Tree Player`))))))

(event `ReportCharge`
  (params (Power :type "Float (double-precision)"))
  ; Charge throw
  (set `self.ThrowPower` Power))

(event `self.ReceiveTick`
  (params (DeltaSeconds :type "Float (single-precision)"))
  (`parent.ReceiveTick` DeltaSeconds)
  (if (`self.isLit`)
    (`KismetSystemLibrary.Delay` 0.1)
    (bind _result (`/Engine/EditorBlueprintResources/StandardMacros.DecrementInt` (`self.InFuse`))
      (:`  `
        (`self.FuseFX` _result)
        (`self.ReportFuse` _result)))))

(event `/Game/Blueprints/DodgeBombs/BPI_DodgeBomb.Transfer`
  (params (Type :type "/Game/Blueprints/DodgeBombs/E_BombType Enum" :default "NewEnumerator0") (Fuse :type Integer) (Age :type "Float (double-precision)") (Parent :type "Actor Object Reference") (IsLit :type Boolean))
  (bind _output_get (set `self.BombToThrow` Type))
  (switch `/Game/Blueprints/DodgeBombs/E_BombType` _output_get
    (:`NewEnumerator0`
      (`self.SetModelNormal` :!label _label_2)
      (set `self.SuperThrow` false))
    (:`NewEnumerator1`
      (goto _label_2))
    (:`NewEnumerator2`
      (`self.SetModelNuke`)
      (set `self.SuperThrow` true))
    (:`NewEnumerator3`
      (set `self.SuperThrow` false)
      (`self.SetModelDrone`)))
  (`/Game/DoubleAction/FirstPerson/Blueprints/BPI_PlayerStatsAndSaving.AddHealth` (`self.As BP State Tree Player`) 30.0)
  (bind _output_get_2 (set `self.InFuse` Fuse))
  (set `/Game/DoubleAction/FirstPerson/Blueprints/BP_StateTreePlayer.IsHoldingBomb` true (`self.As BP State Tree Player`))
  (set `self.HasBomb` true)
  (`KismetSystemLibrary.PrintText` (`|FormatText` "Picking up Bomb with {fuse} Fuse" (`KismetMathLibrary.Conv_IntToDouble` _output_get_2)))
  (`self.FuseFX` (`self.InFuse`))
  (`SceneComponent.SetVisibility` (`self.StaticMesh`) true false)
  (`self.cookBomb`))

(event `ReportFuse`
  (params (Fuse :type Integer))
  (bind _defaultsceneroot (`self.DefaultSceneRoot`))
  ; Explode if overcooked
  (`KismetSystemLibrary.PrintString` (`KismetStringLibrary.Conv_IntToString` Fuse))
  (if (<= Fuse 0)
    ;; only explode if i am still holding bomb
    (if (`self.HasBomb`)
      (`|SpawnActorFromClass` "/Game/Blueprints/DodgeBombs/BP_Explosion.BP_Explosion_C" (`KismetMathLibrary.MakeTransform` (+ (`SceneComponent.K2_GetComponentLocation` _defaultsceneroot) (`SceneComponent.GetForwardVector` _defaultsceneroot)) (`SceneComponent.K2_GetComponentRotation` _defaultsceneroot)) "Undefined" "MultiplyWithRoot" null self (`self.GetInstigator`))
      (`self.LoseBomb`))))

(event `FuseFX`
  (params (Fuse :type Integer))
  (bind _returnvalue (`KismetMathLibrary.MapRangeClamped` (`KismetMathLibrary.Conv_IntToDouble` Fuse) 0.0 29.0 1.0))
  ; Explode if overcooked
  (`MeshComponent.SetScalarParameterValueOnMaterials` (`self.StaticMesh`) "Fuse" _returnvalue)
  (if (== (mod Fuse 2) 0)
    (bind _returnvalue_2 (`GameplayStatics.SpawnSound2D` "/Game/Audio/SC_TickingBomb.SC_TickingBomb" 1.0 1.0 0.0 null))
    (`AudioParameterControllerInterface.SetFloatParameter` _returnvalue_2 "Blend" _returnvalue)))

(event `LoseBomb`
  (`self.Open hands`)
  (`MeshComponent.SetScalarParameterValueOnMaterials` (`self.StaticMesh`) "Fuse" 0.0)
  (set `self.isLit` false)
  (set `/Game/DoubleAction/FirstPerson/Blueprints/BP_StateTreePlayer.IsHoldingBomb` false (`self.As BP State Tree Player`))
  (set `self.HasBomb` false)
  (`SceneComponent.SetVisibility` (`self.StaticMesh`) false false))

(event `SetModelNormal`
  (bind _staticmesh (`self.StaticMesh`))
  (`PrimitiveComponent.SetMaterial` _staticmesh 0 "/Game/Materials/M_DogeBall.M_DogeBall")
  (`StaticMeshComponent.SetStaticMesh` _staticmesh "/Engine/VREditor/BasicMeshes/SM_Ball_01.SM_Ball_01")
  (`SceneComponent.SetRelativeScale3D` (`self.StaticMesh`) (0.3 0.3 0.3)))

(event `Try To catch Bomb`
  ;[0.15 0.139 0.06097 0.5] Catching Bomb
  ;; CatchingBomb
  (`GameplayStatics.PlaySound2D` "/Game/Audio/SFX/WallaceToySFX/04_Swoosh/Swoosh_Down.Swoosh_Down" 1.0 1.0 0.0 null null)
  (if (not (`self.HasBomb`))
    (`/Engine/EditorBlueprintResources/StandardMacros.DoOnce` false :!label _label_3
      (:`Completed`
        (bind (_didhit _bomb) (`self.TraceForBombs`))
        (if _didhit
          (message `/Game/Blueprints/DodgeBombs/BPI_DodgeBomb.MayIPickYouUp` _bomb self)
          (else
            (`KismetSystemLibrary.DelayUntilNextTick`)
            (`self.LoseBomb`)))))))

(event `SetModelDrone`
  (`PrimitiveComponent.SetMaterial` (`self.StaticMesh`) 0 "/Game/Materials/M_DogeBall.M_DogeBall")
  (`StaticMeshComponent.SetStaticMesh` (`self.StaticMesh`) "/Game/Characters/NAC_LowPoly/SM_NacHead.SM_NacHead")
  (`SceneComponent.SetRelativeScale3D` (`self.StaticMesh`) (0.7 0.7 0.7))
  (`KismetSystemLibrary.DelayUntilNextTick`)
  (set `self.isLit` false))

(event `SetModelNuke`
  (`PrimitiveComponent.SetMaterial` (`self.StaticMesh`) 0 "/Game/Materials/M_DogeBall.M_DogeBall")
  (`StaticMeshComponent.SetStaticMesh` (`self.StaticMesh`) "/Game/Blueprints/DodgeBombs/Models/SM_NuclearFootball.SM_NuclearFootball")
  (`SceneComponent.SetRelativeScale3D` (`self.StaticMesh`) (0.3 0.3 0.3))
  (`KismetSystemLibrary.DelayUntilNextTick`)
  (set `self.isLit` false))

(event `Open hands`
  ;[0.15 0.139 0.06097 0.5] Catching Bomb
  (goto _label_3 :!via `Reset`))

(fn `TraceForBombs`
  (returns (DidHit :type Boolean) (Bomb :type "Actor Object Reference"))
  (bind _firstpersoncamera (`/Game/DoubleAction/FirstPerson/Blueprints/BP_StateTreePlayer.FirstPersonCamera` (`self.As BP State Tree Player`)))
  (bind _outactors (`KismetSystemLibrary.SphereOverlapActors` (+ (* (`SceneComponent.GetForwardVector` _firstpersoncamera) 100.0) (`SceneComponent.K2_GetComponentLocation` _firstpersoncamera)) 200.0 (`self.Object Types`) "/Game/Blueprints/DodgeBombs/BP_Grenade.BP_Grenade_C"))
  (if (> (`KismetArrayLibrary.Array_Length` _outactors) 0)
    (return true (`|GetArrayItem` _outactors))
    (else
      (return false null))))

(fn `UserConstructionScript`
  (set `self.Yoffset` 1000.0)
  (set `self.LetMeshDecideBounds` true)
  (`parent.UserConstructionScript`))