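; Throwable dodgeball bomb in three types (bomb, nuke, suicide spawner) that either lies idle as a physics object or flies as an optionally homing projectile.
; A Delay-throttled Tick counts down thrown fuses, driving material, ticking sound and AI noise, while impact types explode after bouncing.
; Bounces deal speed-based knockback and damage, or detonate on bombs and bomb carriers.
; Detonation spawns an explosion or suicide enemy, while pickup passes type and fuse on.
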(event `self.ReceiveTick`
  (params (DeltaSeconds :type "Float (single-precision)"))
  (bind _returnvalue (`KismetMathLibrary.MapRangeClamped` (`KismetMathLibrary.Conv_IntToDouble` (`self.LitFuse`)) 0.0 29.0 1.0))
  ; Fuse
  ;; "is Fuse Lit"
  (if (`self.SpawnIdle`)
    (`self.No longer safe`)
    (elif (not (`self.IsImpact`))
      (`KismetSystemLibrary.Delay` 0.1)
      (bind _result (`/Engine/EditorBlueprintResources/StandardMacros.DecrementInt` (`self.LitFuse`))
        (:`  `
          (`MeshComponent.SetScalarParameterValueOnMaterials` (`self.Sphere1`) "Fuse" _returnvalue)
          (if (== (mod _result 4) 0)
            (bind _returnvalue_2 (`GameplayStatics.SpawnSoundAttached` "/Game/Audio/SC_TickingBomb.SC_TickingBomb" (`self.Sphere`) "None" (0.0 0.0 0.0) (struct) "KeepRelativeOffset" false 1.0 1.0 0.0 null null))
            (`/Engine/EditorBlueprintResources/StandardMacros.IsValid` _returnvalue_2
              (:`Is Valid`
                (`AudioParameterControllerInterface.SetFloatParameter` _returnvalue_2 "Blend" _returnvalue)
                (`self.MakeNoise` 3.0 (`GameplayStatics.GetPlayerPawn` 0) (`SceneComponent.K2_GetComponentLocation` (`self.Sphere`))))))
          (if (<= (`self.LitFuse`) 0)
            (`self.Splode`)))))))

(event `No longer safe`
  (bind _tag_container (`self.Tag Container`))
  (if (<= (`self.LitFuse`) 5)
    (`/Engine/EditorBlueprintResources/StandardMacros.DoOnce` false
      (:`Completed`
        (`BlueprintGameplayTagLibrary.RemoveGameplayTag` _tag_container (struct :`TagName` "Risk.High"))
        (`BlueprintGameplayTagLibrary.AddGameplayTag` _tag_container (struct :`TagName` "Risk.Severe"))))
    (elif (<= (`self.LitFuse`) 15)
      (`/Engine/EditorBlueprintResources/StandardMacros.DoOnce` false
        (:`Completed`
          (`BlueprintGameplayTagLibrary.RemoveGameplayTag` _tag_container (struct :`TagName` "Risk.Medium"))
          (`BlueprintGameplayTagLibrary.AddGameplayTag` _tag_container (struct :`TagName` "Risk.High"))))
      (elif (<= (`self.LitFuse`) 25)
        (`/Engine/EditorBlueprintResources/StandardMacros.DoOnce` false
          (:`Completed`
            (`BlueprintGameplayTagLibrary.RemoveGameplayTag` _tag_container (struct :`TagName` "Risk.Low"))
            (`BlueprintGameplayTagLibrary.AddGameplayTag` _tag_container (struct :`TagName` "Risk.Medium"))))))))

(event `Splode`
  (bind _returnvalue (`GameplayStatics.GetPlayerPawn` 0))
  ; Explode
  (switch `/Game/Blueprints/DodgeBombs/E_BombType` (`self.BombType`)
    (:`NewEnumerator1`
      (`|SpawnActorFromClass` "/Game/Blueprints/DodgeBombs/BP_Explosion.BP_Explosion_C" (`KismetMathLibrary.Conv_VectorToTransform` (`self.K2_GetActorLocation`)) "Undefined" "MultiplyWithRoot" null self _returnvalue :!label _label)
      (`self.K2_DestroyActor`))
    (:`NewEnumerator2`
      (`|SpawnActorFromClass` "/Game/Blueprints/DodgeBombs/BP_Explosion_Nuke.BP_Explosion_Nuke_C" (`KismetMathLibrary.Conv_VectorToTransform` (`self.K2_GetActorLocation`)) "Undefined" "MultiplyWithRoot" null self _returnvalue)
      (`self.K2_DestroyActor`))
    (:`NewEnumerator3`
      (if (`self.SpawnIdle`)
        (goto _label)
        (elif (== (`self.LastOwner`) (`GameplayStatics.GetPlayerPawn` 0))
          (`|SpawnActorFromClass` "/Game/AI_Blueprints/BP_SuicideEnemyGoodGuy.BP_SuicideEnemyGoodGuy_C" (`KismetMathLibrary.Conv_VectorToTransform` (`self.K2_GetActorLocation`)) "Undefined" "MultiplyWithRoot" null (`GameplayStatics.GetPlayerPawn` 0))
          (`self.K2_DestroyActor`)
          (else
            (`|SpawnActorFromClass` "/Game/AI_Blueprints/BP_SuicideEnemyPrimed.BP_SuicideEnemyPrimed_C" (`KismetMathLibrary.Conv_VectorToTransform` (`self.K2_GetActorLocation`)) "Undefined" "MultiplyWithRoot" null (`self.GetInstigator`))
            (`self.K2_DestroyActor`)))))))

(event `self.ReceiveAnyDamage`
  (params (Damage :type "Float (single-precision)") (DamageType :type "DamageType Object Reference") (InstigatedBy :type "Controller Object Reference") (DamageCauser :type "Actor Object Reference"))
  ; there is no reason why this should break unreal but it does
  (if (`self.CanBeDamaged`)
    (`KismetSystemLibrary.Delay` 0.2)
    (`self.Splode`)))

(event `self.ReceiveBeginPlay`
  (bind _homingtarget (`self.HomingTarget`))
  (bind _sphere (`self.Sphere`))
  (bind _sphere1 (`self.Sphere1`))
  (bind _projectilemovement (`self.ProjectileMovement`))
  (bind _sphere1_2 (`self.Sphere1`))
  (bind _initialspeed (`self.initialSpeed`))
  ; Begin Play
  ;; Player gets a bigger projectile
  (if (== (`self.LastOwner`) (`GameplayStatics.GetPlayerPawn` 0))
    (`SphereComponent.SetSphereRadius` _sphere 50.0 true)
    (else
      (`SphereComponent.SetSphereRadius` _sphere 29.0 true)))
  (switch `/Game/Blueprints/DodgeBombs/E_BombType` (`self.BombType`)
    (:`NewEnumerator0`
      (`SceneComponent.SetRelativeScale3D` _sphere1 (0.4 0.4 0.4) :!label _label_2))
    (:`NewEnumerator1`
      (goto _label_2))
    (:`NewEnumerator2`
      (`StaticMeshComponent.SetStaticMesh` _sphere1 "/Game/Blueprints/DodgeBombs/Models/SM_NuclearFootball.SM_NuclearFootball")
      (`SceneComponent.SetRelativeScale3D` _sphere1 (0.6 0.6 0.6))
      (set `self.IsImpact` true)
      (set `self.bCanBeDamaged` false) ; keeps accidentally getting set off
    )
    (:`NewEnumerator3`
      ;; Player Throws Friendlys
      (set `self.CanBeDamaged` false)
      (if (== (`self.LastOwner`) (`GameplayStatics.GetPlayerPawn` 0))
        (set `self.IsImpact` true))
      (`StaticMeshComponent.SetStaticMesh` _sphere1_2 "/Game/Characters/NAC_LowPoly/SM_NacHead.SM_NacHead")
      (`SceneComponent.SetRelativeScale3D` _sphere1_2 (1.0 1.0 1.0))))
  (`GameplayStatics.SpawnSoundAttached` "/Game/Audio/SC_BallThrow.SC_BallThrow" (`self.Sphere`) "None" (0.0 0.0 0.0) (struct) "KeepRelativeOffset" false 1.0 1.0 0.0 null null)
  (if (`self.SpawnIdle`)
    (`PrimitiveComponent.SetSimulatePhysics` (`self.Sphere`) true)
    (set `self.LitFuse` 30)
    (`BlueprintGameplayTagLibrary.AddGameplayTag` (`self.Tag Container`) (struct :`TagName` "Risk.Medium"))
    (else
      (if (`KismetSystemLibrary.IsValid` _homingtarget)
        (set `ProjectileMovementComponent.HomingTargetComponent` (`self.GetParentComponent` _homingtarget) (`self.ProjectileMovement`))
        (else
          (set `ProjectileMovementComponent.bIsHomingProjectile` false (`self.ProjectileMovement`))))
      (`PrimitiveComponent.SetSimulatePhysics` (`self.Sphere`) false)
      (bind _output_get (set `ProjectileMovementComponent.InitialSpeed` _initialspeed _projectilemovement))
      ;; For Homing
      (set `ProjectileMovementComponent.MaxSpeed` _initialspeed _projectilemovement)
      (`ProjectileMovementComponent.SetVelocityInLocalSpace` (`self.ProjectileMovement`) (`KismetMathLibrary.MakeVector` _output_get))
      (set `self.LitFuse` (+ (`KismetMathLibrary.FTrunc` (* (`self.Fuse`) 10.0)) 1)))))

(event `/Game/Blueprints/DodgeBombs/BPI_DodgeBomb.MayIPickYouUp`
  (params (Me :type "Actor Object Reference"))
  (message `/Game/Blueprints/DodgeBombs/BPI_DodgeBomb.Transfer` Me (`self.BombType`) (`self.LitFuse`) 0.0 (`self.LastOwner`) (!= (`self.SpawnIdle`) true))
  (`self.K2_DestroyActor`))

(event `self.ProjectileMovement.OnProjectileBounce`
  (params (ImpactResult :type "HitResult Structure (by ref)") (ImpactVelocity :type "Vector Structure (by ref)"))
  (bind _returnvalue (`GameplayStatics.GetPlayerPawn` 0))
  (bind _returnvalue_2 (`KismetMathLibrary.VSize` ImpactVelocity))
  (bind (_bblockinghit _binitialoverlap _time _distance _location _impactpoint _normal _impactnormal _physmat _hitactor) (`GameplayStatics.BreakHitResult` ImpactResult))
  (bind _returnvalue_3 (> (`self.i`) 3))
  (bind _returnvalue_4 (* _normal (* _returnvalue_2 -1.0)))
  ; Damaging
  (if (`self.IsImpact`)
    (`|ExecutionSequence`
      (:`then_0`
        ;; Splode when hitting other bombs
        (cast `/Game/Blueprints/DodgeBombs/BP_Grenade` _hitactor :!label _label_3
          (:`then`
            (`self.Splode`))
          (:`CastFailed`
            (bind _asbp_enemy_base (cast `/Game/AI_Blueprints/BP_EnemyBase` _hitactor)
              (:`then`
                (if (`/Game/AI_Blueprints/BP_EnemyBase.IsHoldingBomb` _asbp_enemy_base)
                  (`self.Splode`)
                  (else
                    (bind _asbp_state_tree_player (cast `/Game/DoubleAction/FirstPerson/Blueprints/BP_StateTreePlayer` _hitactor :!label _label_4)
                      (:`then`
                        (if (`/Game/DoubleAction/FirstPerson/Blueprints/BP_StateTreePlayer.IsHoldingBomb` _asbp_state_tree_player)
                          (`self.Splode`)
                          (else
                            (if (> (`self.i`) 0) :!label _label_5
                              (`/Engine/EditorBlueprintResources/StandardMacros.DecrementInt` (`self.i`)
                                (:`  `
                                  (if (> _returnvalue_2 5500.0)
                                    (`self.MakeNoise` 3.0 _returnvalue)
                                    (`GameplayStatics.SpawnSoundAtLocation` "/Game/Audio/ViolentDodgeBall_Cue.ViolentDodgeBall_Cue" (`SceneComponent.K2_GetComponentLocation` (`self.Sphere1`)) (struct) 1.0 1.0 0.0 null null)
                                    (if _returnvalue_3
                                      (set `self.knock` (* _returnvalue_4 2.0))
                                      (set `self.Damage` 50.0)
                                      (`/Engine/EditorBlueprintResources/StandardMacros.IsValid` _hitactor :!label _label_6
                                        (:`Is Valid`
                                          (bind _ascharacter (cast `Character` _hitactor)
                                            (:`then`
                                              (`CharacterMovementComponent.AddImpulse` (`Character.CharacterMovement` _ascharacter) (`self.knock`) true))
                                            (:`CastFailed`
                                              _))
                                          (`GameplayStatics.ApplyPointDamage` _hitactor (`self.Damage`) _impactpoint ImpactResult))))
                                    (else
                                      (`self.MakeNoise` 1.0 _returnvalue _impactpoint)
                                      (`GameplayStatics.SpawnSoundAttached` "/Game/Audio/CopyInfDodgeball_Cue.CopyInfDodgeball_Cue" (`self.Sphere1`) "None" (0.0 0.0 0.0) (struct) "SnapToTarget" false (`KismetMathLibrary.MapRangeClamped` _returnvalue_2 1.0 4000.0 0.01 1.0) 1.0 0.0 null null)
                                      (if _returnvalue_3
                                        (set `self.knock` (* _returnvalue_4 0.5))
                                        (set `self.Damage` 30.0)
                                        (goto _label_6))))))))))
                      (:`CastFailed`
                        (goto _label_5))))))
              (:`CastFailed`
                (goto _label_4))))))
      (:`then_1`
        (`KismetSystemLibrary.Delay` 0.2)
        (`self.Splode`)))
    (else
      (goto _label_3))))

(fn `UserConstructionScript`
  (if (`self.SpawnIdle`)
    (`BlueprintGameplayTagLibrary.AddGameplayTag` (`self.Tag Container`) (struct :`TagName` "Risk.Low"))))

(fn `WhachaFuseAt`
  (returns (CeilFuse :type Integer))
  (return (`self.LitFuse`)))