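; One-shot explosion actor for DodgeBombs that damages and knocks back what it reaches, then destroys itself after a short delay.
; On spawn it emits AI noise, effects, sound and force feedback, then sphere-traces its radius, keeping one hit per actor.
; Line traces back to the origin filter out occluded actors.
; Survivors receive distance-scaled point damage and radial physics force, with Characters getting additional falloff-based damage and movement impulse.
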(event `self.ReceiveBeginPlay`
  (bind _origin (`self.Origin`))
  ; explosion
  (bind _output_get (set `self.Origin` (`SceneComponent.K2_GetComponentLocation` (`self.DefaultSceneRoot`))))
  (`self.MakeNoise` 3.0 (`GameplayStatics.GetPlayerPawn` 0) _output_get)
  (`NiagaraFunctionLibrary.SpawnSystemAtLocation` (`self.System Template`) _output_get)
  (`GameplayStatics.PlaySoundAtLocation` (`self.Sound`) _output_get (struct) (`self.Volume`) (`self.Pitch`) 0.0 null null null null)
  (`GameplayStatics.SpawnForceFeedbackAtLocation` "/Game/DoubleAction/FirstPerson/Blueprints/FFB_GroundPound.FFB_GroundPound" _output_get (struct) false 1.0 0.0 "/Game/LeastOfThese/BluePrints/FX/Rumble/FFA_SmallPhys1.FFA_SmallPhys1")
  (bind _outhits (`KismetSystemLibrary.SphereTraceMultiByProfile` _origin _origin (`self.DamageRadius`) "BlockAll"))
  ;; There are multiple hits per actor, include each actor once
  (for _array_element _outhits
    (bind (_bblockinghit _binitialoverlap _time _distance _location _impactpoint _normal _impactnormal _physmat _hitactor) (`GameplayStatics.BreakHitResult` _array_element))
    (if (`KismetArrayLibrary.Array_Contains` (`self.Array Element Hit Actor`) _hitactor)
      (`KismetSystemLibrary.Delay` 0.1)
      (`self.K2_DestroyActor`)
      (else
        (`KismetArrayLibrary.Array_Add` (`self.Array Element Hit Actor`) _hitactor)
        (`KismetArrayLibrary.Array_Add` (`self.GoodHits`) _array_element))))
  ;; Explosion Occlusion
  (for _array_element_2 (`self.GoodHits`)
    (bind (_bblockinghit_2 _binitialoverlap_2 _time_2 _distance_2 _location_2 _impactpoint_2 _normal_2 _impactnormal_2 _physmat_2 _hitactor_2) (`GameplayStatics.BreakHitResult` _array_element_2))
    (bind (_outhit _returnvalue) (`KismetSystemLibrary.LineTraceSingleByProfile` (+ _impactpoint_2 (* _normal_2 50.0)) (`self.Origin`) "BlockAll" false (`|MakeArray` _hitactor_2 (`self.Creator`)) "None" true (struct :`R` 0.04883 :`G` 1.0 :`A` 1.0) (struct :`R` 1.0 :`G` 0.064089 :`A` 1.0)))
    ;;; If the is no blocking hit, then the explosion got us. using aray so occlusion still works.
    (if (not _returnvalue)
      (`KismetArrayLibrary.Array_Add` (`self.FinalHits`) _array_element_2)))
  (if (> (`KismetArrayLibrary.Array_Length` (`self.FinalHits`)) 0)
    ;; Damage
    (for _array_element_3 (`self.FinalHits`)
      (`self.DagageCharacters` _array_element_3)
      (`self.Impulse Physics` _array_element_3)
      (bind (_bblockinghit_3 _binitialoverlap_3 _time_3 _distance_3 _location_3 _impactpoint_3 _normal_3 _impactnormal_3 _physmat_3 _hitactor_3 _hitcomponent _hitbonename _bonename _hititem _elementindex _faceindex _tracestart _traceend) (`GameplayStatics.BreakHitResult` _array_element_3))
      (`GameplayStatics.ApplyPointDamage` _hitactor_3 (`KismetMathLibrary.MapRangeClamped` (`KismetMathLibrary.Vector_Distance` _tracestart _traceend) 0.0 (`self.DamageRadius`) 5.0 (`self.Damage`)) _impactnormal_3 _array_element_3 (`self.GetInstigatorController`) (`self.Creator`)))
    (`KismetSystemLibrary.Delay` 0.1)
    (`self.K2_DestroyActor`)
    (else
      (`KismetSystemLibrary.Delay` 0.1)
      (`self.K2_DestroyActor`))))

(event `DagageCharacters`
  (params (hit :type "HitResult Structure"))
  (bind (_bblockinghit _binitialoverlap _time _distance _location _impactpoint _normal _impactnormal _physmat _hitactor) (`GameplayStatics.BreakHitResult` hit))
  (bind _damageradius (`self.DamageRadius`))
  (bind _returnvalue (`KismetMathLibrary.MapRangeClamped` (- _damageradius (`KismetMathLibrary.Vector_Distance` (`self.K2_GetActorLocation`) (`self.K2_GetActorLocation` _hitactor))) 0.0 _damageradius 0.0 1.0))
  ; explosion
  ;; Unreal thinks this is an infinite loop, but only some times
  ;; Radial Fall off For Character pawns
  (bind _ascharacter (cast `Character` _hitactor))
  (`CharacterMovementComponent.AddImpulse` (`Character.CharacterMovement` _ascharacter) (* _normal (* (* (`self.KnockBack`) -1.0) _returnvalue)) true)
  (`GameplayStatics.ApplyPointDamage` _ascharacter (* _returnvalue (`self.Damage`)) _normal hit null (`self.GetInstigator`)))

(event `Impulse Physics`
  (params (hit :type "HitResult Structure"))
  ; explosion
  ;; impulse for physics objects
  (`PrimitiveComponent.AddRadialForce` (`.HitComponent` (`GameplayStatics.BreakHitResult` hit)) (- (`self.K2_GetActorLocation`) (0.0 0.0 50.0)) (`self.DamageRadius`) (* (`self.KnockBack`) 30.0) "RIF_Linear" true))

(fn `UserConstructionScript`
  (`SphereComponent.SetSphereRadius` (`self.Sphere`) (`self.DamageRadius`) true))