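; Bomb pedestal for the DodgeBombs game that launches a BP_GrenadeSafe of its configured BombType from its Sphere's transform.
; BeginPlay waits a random few seconds, plays a burst effect and launcher sound, then spawns the grenade and stores it as MyBaby.
; Tick uses latent Delays as a polling timer: once MyBaby is invalid, a random wait and coin flip decide whether to repeat the spawn sequence.
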(event `self.ReceiveBeginPlay`
  (bind _returnvalue (`SceneComponent.K2_GetComponentToWorld` (`self.Sphere`)))
  (bind _location (.location _returnvalue))
  (`KismetSystemLibrary.Delay` (`KismetMathLibrary.Conv_Int64ToDouble` (`KismetMathLibrary.RandomInteger64InRange` 0 5)))
  (`NiagaraFunctionLibrary.SpawnSystemAtLocation` "/Niagara/DefaultAssets/Templates/Systems/DirectionalBurst.DirectionalBurst" _location :!label _label)
  (`GameplayStatics.PlaySoundAtLocation` "/Game/Audio/SFX/WallaceToySFX/00_Toys/Toy_GrenadeLauncher.Toy_GrenadeLauncher" _location (struct) 2.0 1.0 0.0 "/Game/Audio/Attenuation/SA_PhysicsImpact.SA_PhysicsImpact" null null null)
  (`KismetSystemLibrary.Delay` 0.2)
  (bind _returnvalue_2 (`|SpawnActorFromClass` "/Game/Blueprints/DodgeBombs/BP_GrenadeSafe.BP_GrenadeSafe_C" _returnvalue "Undefined" "MultiplyWithRoot" null 5.0 0.0 false null (`self.BombType`) null null))
  (set `self.MyBaby` _returnvalue_2))

(event `self.ReceiveTick`
  (params (DeltaSeconds :type "Float (single-precision)"))
  (`KismetSystemLibrary.Delay` 4.0)
  (if (not (`KismetSystemLibrary.IsValid` (`self.MyBaby`)))
    (`KismetSystemLibrary.Delay` (`KismetMathLibrary.Conv_Int64ToDouble` (`KismetMathLibrary.RandomInteger64InRange` 0 5)))
    (if (`KismetMathLibrary.RandomBool`)
      (goto _label))))

(fn `UserConstructionScript`)