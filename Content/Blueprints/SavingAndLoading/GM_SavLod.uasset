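; Game mode that saves and loads player stats and per-level state, loading both on BeginPlay.
; Player stats live in the "PlayerSave" slot and are copied onto the third-person character's stamina, health and mana.
; Level state uses the level name as its slot, replaying collected coins and opened doors on load.
; Missing saves get fresh objects; save events write the held objects to disk without gathering values themselves.
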(event `self.ReceiveBeginPlay`
  (`KismetSystemLibrary.PrintString` "Loaded in SaveLoad Game Mode" true true (struct :`R` 1.0 :`B` 0.90722 :`A` 1.0) 10.0)
  (`self.LoadPlayerStats`)
  (`self.Load level State`))

(event `LoadPlayerStats`
  (bind _sg_playerstats (`self.SG_PlayerStats`))
  (bind _returnvalue (`GameplayStatics.DoesSaveGameExist` "PlayerSave"))
  (if _returnvalue
    (bind _returnvalue_2 (`GameplayStatics.LoadGameFromSlot` "PlayerSave"))
    (bind _assg_player_stats (cast `/Game/Blueprints/SavingAndLoading/SG_PlayerStats` _returnvalue_2))
    (set `self.SG_PlayerStats` _assg_player_stats)
    (bind _asbp_third_person_character (cast `/Game/ThirdPerson/Blueprints/BP_ThirdPersonCharacter` (`GameplayStatics.GetPlayerCharacter` 0)))
    (set `/Game/ThirdPerson/Blueprints/BP_ThirdPersonCharacter.Stamina` (`/Game/Blueprints/SavingAndLoading/SG_PlayerStats.Stamina` _sg_playerstats) _asbp_third_person_character)
    (set `/Game/ThirdPerson/Blueprints/BP_ThirdPersonCharacter.Health` (`/Game/Blueprints/SavingAndLoading/SG_PlayerStats.Health` _sg_playerstats) _asbp_third_person_character)
    (set `/Game/ThirdPerson/Blueprints/BP_ThirdPersonCharacter.manna` (`/Game/Blueprints/SavingAndLoading/SG_PlayerStats.Mana` _sg_playerstats) _asbp_third_person_character)
    (`KismetSystemLibrary.PrintString` "Player stats have been loaded")
    (else
      (bind _returnvalue_3 (`GameplayStatics.CreateSaveGameObject` "/Game/Blueprints/SavingAndLoading/SG_PlayerStats.SG_PlayerStats_C"))
      (set `self.SG_PlayerStats` _returnvalue_3))))

(event `save player stats`
  (bind _returnvalue (`GameplayStatics.SaveGameToSlot` (`self.SG_PlayerStats`) "PlayerSave"))
  (if _returnvalue
    (`KismetSystemLibrary.PrintText` "Player stas written to file")
    (else
      (`KismetSystemLibrary.PrintText` "Player stats could not be written to save file" true true (struct :`R` 1.0 :`G` 0.000412 :`A` 1.0)))))

(event `Save Level State`
  (bind _returnvalue (`GameplayStatics.GetCurrentLevelName` true))
  (bind _returnvalue_2 (`GameplayStatics.SaveGameToSlot` (`self.SG_LevelState`) _returnvalue))
  (if _returnvalue_2
    (`KismetSystemLibrary.PrintText` "Level state saved to game file")
    (else
      (`KismetSystemLibrary.PrintText` "Level State not saved!"))))

(event `Load level State`
  (bind _returnvalue (`GameplayStatics.GetCurrentLevelName` true))
  (bind _returnvalue_2 (`GameplayStatics.DoesSaveGameExist` _returnvalue))
  (if _returnvalue_2
    (bind _returnvalue_3 (`GameplayStatics.LoadGameFromSlot` _returnvalue))
    (bind _assg_level_state (cast `/Game/Blueprints/SavingAndLoading/SG_LevelState` _returnvalue_3))
    (bind _output_get (set `self.SG_LevelState` _assg_level_state))
    (`|ExecutionSequence`
      (:`then_0`
        (for _array_element (`/Game/Blueprints/SavingAndLoading/SG_LevelState.CollectedCoins` _output_get)
          (`/Engine/EditorBlueprintResources/StandardMacros.IsValid` _array_element
            (:`Is Valid`
              (`/Game/Blueprints/Pickups/BP_coin.alredy collected` _array_element))))
        (`KismetSystemLibrary.PrintText` "Coin State Loaded"))
      (:`then_1`
        (for _array_element_2 (`/Game/Blueprints/SavingAndLoading/SG_LevelState.OpenedDoors` _output_get)
          (`/Engine/EditorBlueprintResources/StandardMacros.IsValid` _array_element_2
            (:`Is Valid`
              (`/Game/Blueprints/BP_CameraDoor.Soft open` _array_element_2))))
        (`KismetSystemLibrary.PrintText` "DoorStateloaded")))
    (else
      (bind _returnvalue_4 (`GameplayStatics.CreateSaveGameObject` "/Game/Blueprints/SavingAndLoading/SG_LevelState.SG_LevelState_C"))
      (set `self.SG_LevelState` _returnvalue_4))))

(fn `UserConstructionScript`)