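; One-shot explosion actor that fires on BeginPlay and then destroys itself.
; It makes AI noise at the player pawn's instigation, spawns effect and sound, and applies radial damage.
; Sphere overlaps then give Characters linearly distance-scaled knockback and additional damage, and push physics components with radial force from below the origin.
; DamageRadius drives every query and sizes the Sphere component in the construction script.
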(event `self.ReceiveBeginPlay`
  (bind _returnvalue (`self.K2_GetActorLocation`))
  (bind _returnvalue_2 (`self.K2_GetActorLocation`))
  (bind _returnvalue_3 (`self.K2_GetActorLocation`))
  (bind _damageradius (`self.DamageRadius`))
  (bind _damageradius_2 (`self.DamageRadius`))
  ; explosion
  (`self.MakeNoise` 3.0 (`GameplayStatics.GetPlayerPawn` 0) _returnvalue_3)
  (`NiagaraFunctionLibrary.SpawnSystemAtLocation` "/Niagara/DefaultAssets/Templates/Systems/SimpleExplosion.SimpleExplosion" _returnvalue_3)
  (`GameplayStatics.PlaySoundAtLocation` "/Engine/EditorSounds/GamePreview/StartPlayInEditor_Cue.StartPlayInEditor_Cue" (0.0 0.0 0.0) (struct) 1.0 0.8 0.0 null null null null)
  (`GameplayStatics.ApplyRadialDamage` :`BaseDamage` 20.0 :`Origin` _returnvalue_3 :`DamageRadius` _damageradius_2 :`DamageCauser` (`self.GetInstigator`) :`InstigatedByController` null)
  (bind _outactors (`KismetSystemLibrary.SphereOverlapActors` _returnvalue_3 _damageradius_2 (`self.Object Types`)))
  (for _array_element _outactors
    ;; Radial Fall off For Character pawns
    (bind _ascharacter (cast `Character` _array_element))
    (bind _returnvalue_4 (`self.K2_GetActorLocation` _array_element))
    (bind _returnvalue_5 (`KismetMathLibrary.MapRangeClamped` (- _damageradius (`KismetMathLibrary.Vector_Distance` _returnvalue_2 _returnvalue_4)) 0.0 _damageradius 0.0 1.0))
    (`CharacterMovementComponent.AddImpulse` (`Character.CharacterMovement` _ascharacter) (* (`KismetMathLibrary.Conv_RotatorToVector` (`KismetMathLibrary.FindLookAtRotation` _returnvalue_2 _returnvalue_4)) (* (`self.KnockBack`) _returnvalue_5)) true)
    (`GameplayStatics.ApplyDamage` _ascharacter (* _returnvalue_5 (`self.Damage`)) null (`self.GetInstigator`)))
  ;; impulse for physics objects
  (bind _outcomponents (`KismetSystemLibrary.SphereOverlapComponents` _returnvalue (`self.DamageRadius`) (`self.Object Types_0`)))
  (for _array_element_2 _outcomponents
    (`PrimitiveComponent.AddRadialForce` _array_element_2 (- _returnvalue (0.0 0.0 50.0)) (`self.DamageRadius`) (* (`self.KnockBack`) 30.0) "RIF_Linear" true))
  (`self.K2_DestroyActor`))

(fn `UserConstructionScript`
  (`SphereComponent.SetSphereRadius` (`self.Sphere`) (`self.DamageRadius`) true))